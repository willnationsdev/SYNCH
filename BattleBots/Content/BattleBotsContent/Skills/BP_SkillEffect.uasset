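; Base Blueprint for BattleBots skill effects, with a stub Apply and shared helpers for targeting, health changes and grid movement.
; Targets come from the skill's explicit target or a grid-manager radius query, plus TargetAlso, and can be filtered by ally or enemy team.
; DeltaHealth writes clamped health through the skill user's stats.
; Propel builds stepped direction offsets, and ClampLocationToGrid snaps world locations to cells within the grid.
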(fn Apply
  (params (Skill :type BP%20Skill%20Object%20Reference))
  (return false))

(fn GetSkillUsersinField
  (params (SkillBeingUsed :type BP%20Skill%20Object%20Reference))
  (LocalVariables|SetTheSkill SkillBeingUsed)
  ;[1 1 1] Collect all targets into a singular array, regardless of targeting style
  (bind _asbpi_grid_managing_game_mode (Utilities|Casting|CastToBPI_GridManagingGameMode (Variables|Default|GetGameMode))
    (:then
      (bind _gridmanager (Default|GetGridManager _asbpi_grid_managing_game_mode))
      (bind _units (Default|GetUnitsinField _gridmanager (Variables|/Game/BattleBotsContent/Skills/BP_Skill.BP_Skill_C|GetTargetGridLocationX (LocalVariables|GetTheSkill)) (Variables|/Game/BattleBotsContent/Skills/BP_Skill.BP_Skill_C|GetTargetGridLocationY (LocalVariables|GetTheSkill)) (* (Utilities|Struct|BreakBPS_SkillAttributes (Variables|/Game/BattleBotsContent/Skills/BP_Skill.BP_Skill_C|GetSkillAttributes (LocalVariables|GetTheSkill))) 100)))
      (for _array_element _units
        (bind _asbpi_skill_user (Utilities|Casting|CastToBPI_SkillUser _array_element))
        (Utilities|Array|Add (LocalVariables|GetSkillUsersToTarget) _asbpi_skill_user)))
    (:CastFailed
      _))
  (return (LocalVariables|GetSkillUsersToTarget)))

(fn GetSkillUserTargets
  (params (TheSkill :type BP%20Skill%20Object%20Reference))
  (bind _targetskilluser (Variables|/Game/BattleBotsContent/Skills/BP_Skill.BP_Skill_C|GetTargetSkillUser TheSkill))
  ;[1 1 1] If there is no explicit target, then get a target via grid location
  (Utilities|IsValid (Utilities|ToObject(Interface) _targetskilluser)
    (:Is%20Valid
      (Utilities|Array|AddUnique (LocalVariables|GetSkillUsers) _targetskilluser))
    (:Is%20Not%20Valid
      (bind _skillusers (SkillEffect-Utility|GetSkillUsersinField TheSkill))
      (LocalVariables|SetSkillUsers _skillusers)))
  (Utilities|Array|AppendArray (LocalVariables|GetSkillUsers) (Variables|Default|GetTargetAlso))
  (return (LocalVariables|GetSkillUsers)))

(fn DeltaHealth
  (params (SkillUserToAffect :type BPI%20Skill%20User%20Interface) (DeltaCurrentHealth :type Integer))
  ;[1 1 1] Decrease the target's CurrentHealth by the degree of Intensity
  (bind _stats (Default|GetStats SkillUserToAffect))
  (bind _output_get (LocalVariables|SetTempStats _stats))
  (bind _structout (Utilities|Struct|SetmembersinBPS_Stats _output_get (Math|Integer|Clamp(Integer) (+ (.CurrentHealth (Utilities|Struct|BreakBPS_Stats _stats)) DeltaCurrentHealth) 0 (.MaxHealth (Utilities|Struct|BreakBPS_Stats _stats)))))
  (Default|SetStats SkillUserToAffect _structout))

(fn FilterbyValidTarget
  (params (UnfilteredSkillUsers :type Array%20of%20BPI%20Skill%20User%20Interfaces) (TheSkill :type BP%20Skill%20Object%20Reference))
  (bind _sourceskilluser (Variables|/Game/BattleBotsContent/Skills/BP_Skill.BP_Skill_C|GetSourceSkillUser TheSkill))
  ;[1 1 1] For each target to be affected...
  (for _array_element UnfilteredSkillUsers
    ;[1 1 1] Check whether we care what team they are on
    (switch Utilities|FlowControl|Switch|SwitchonEValidSkillTarget (Utilities|Struct|BreakBPS_SkillAttributes (Variables|/Game/BattleBotsContent/Skills/BP_Skill.BP_Skill_C|GetSkillAttributes TheSkill))
      (:NewEnumerator0
        (Utilities|Array|Add (LocalVariables|GetSkillUsersToReturn) _array_element :!label _label))
      (:NewEnumerator1
        ;[1 1 1] Targets...(TOP) all units, (MID) same-team units, (BOT) other-team units
        (bind _team (Default|GetTeam _sourceskilluser))
        (bind _team_2 (Default|GetTeam _array_element))
        (if (Utilities|Enum|Equal(Enum) _team _team_2)
          (goto _label)))
      (:NewEnumerator2
        (bind _team_3 (Default|GetTeam _sourceskilluser))
        (bind _team_4 (Default|GetTeam _array_element))
        (if (Utilities|Enum|NotEqual(Enum) _team_4 _team_3)
          (goto _label)))))
  (return false (LocalVariables|GetSkillUsersToReturn)))

(fn Propel
  (params (SourceLocation :type Vector) (TargetLocation :type Vector) (PropelAmount :type Integer))
  (for _index (range 1 PropelAmount)
    (Utilities|Array|Add (LocalVariables|GetPropellVectors) (* (* (Class|KismetMathLibrary|GetDirectionVector SourceLocation TargetLocation) 100) _index)))
  (return (LocalVariables|GetPropellVectors)))

(fn ClampLocationtoGrid
  (params (MoveToLocation :type Vector))
  (bind (_x _y _z) (Math|Vector|BreakVector MoveToLocation))
  (bind _asbpi_grid_managing_game_mode (Utilities|Casting|CastToBPI_GridManagingGameMode (Variables|Default|GetGameMode)))
  (bind _gridmanager (Default|GetGridManager _asbpi_grid_managing_game_mode))
  (return (Math|Vector|MakeVector (* (.ClampedMoveToX (Default|ClamptoGridCoordinates _gridmanager (Math|Float|Round (/ _x (Variables|/Game/BattleBotsContent/Grid/BP_GridManager.BP_GridManager_C|GetCellSize _gridmanager))) (Math|Float|Round (/ _y (Variables|/Game/BattleBotsContent/Grid/BP_GridManager.BP_GridManager_C|GetCellSize _gridmanager))))) (Variables|/Game/BattleBotsContent/Grid/BP_GridManager.BP_GridManager_C|GetCellSize _gridmanager)) (* (.ClampedMoveToY (Default|ClamptoGridCoordinates _gridmanager (Math|Float|Round (/ _x (Variables|/Game/BattleBotsContent/Grid/BP_GridManager.BP_GridManager_C|GetCellSize _gridmanager))) (Math|Float|Round (/ _y (Variables|/Game/BattleBotsContent/Grid/BP_GridManager.BP_GridManager_C|GetCellSize _gridmanager))))) (Variables|/Game/BattleBotsContent/Grid/BP_GridManager.BP_GridManager_C|GetCellSize _gridmanager)) _z)))