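; TeleSwap skill effect that swaps the grid positions of the skill's target and a random teammate of the caster.
; Apply gets the grid manager from the game mode, shuffles the caster's teammates, takes the first, and records both units' grid coordinates.
; It clears both cells, parks the target at (0,0), then places each unit at the other's old spot.
; Apply returns false on every path, including a successful swap.
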(fn Apply
  (params (Skill :type BP%20Skill%20Object%20Reference))
  (bind _asbpi_grid_managing_game_mode (Utilities|Casting|CastToBPI_GridManagingGameMode (Variables|Default|GetGameMode))
    (:then
      (bind _gridmanager (Default|GetGridManager _asbpi_grid_managing_game_mode))
      (LocalVariables|SetTheGrid _gridmanager)
      (bind _asbp_unit (Utilities|Casting|CastToBP_Unit (Variables|/Game/BattleBotsContent/Skills/BP_Skill.BP_Skill_C|GetSourceSkillUser Skill))
        (:then
          (bind _output_get (LocalVariables|SetUnitSelf _asbp_unit))
          (bind _teamarray (Default|GetTeamMates (Variables|/Game/BattleBotsContent/Units/BP_Unit.BP_Unit_C|GetBP_UnitTeamComponent _output_get)))
          (if (> (Utilities|Array|Length _teamarray) 0)
            (bind _output_get_2 (LocalVariables|SetTargets _teamarray))
            (Utilities|Array|Shuffle _output_get_2)
            (bind _asbp_unit_2 (Utilities|Casting|CastToBP_Unit (Variables|/Game/BattleBotsContent/Skills/BP_Skill.BP_Skill_C|GetTargetSkillUser Skill))
              (:then
                (Utilities|IsValid _asbp_unit_2
                  (:Is%20Valid
                    (LocalVariables|SetEnUnit _asbp_unit_2)
                    (bind _gridcell (Default|GetGridCellfromObject (LocalVariables|GetTheGrid) (LocalVariables|GetEnUnit)))
                    (LocalVariables|SetNewTeamLoc (Math|Vector|MakeVector (Math|Conversions|ToFloat(Integer) (.GridLocationX (Default|WorldtoGridCoordinates (LocalVariables|GetTheGrid) (Transformation|GetActorLocation _asbp_unit_2)))) (Math|Conversions|ToFloat(Integer) (.GridLocationY (Default|WorldtoGridCoordinates (LocalVariables|GetTheGrid) (Transformation|GetActorLocation _asbp_unit_2)))) 0.0))
                    (Variables|/Game/BattleBotsContent/Grid/BP_GridCell.BP_GridCell_C|SetUnit _gridcell 0)
                    (bind _gridcell_2 (Default|GetGridCellfromObject (LocalVariables|GetTheGrid) (Utilities|Array|Get(acopy) (LocalVariables|GetTargets))))
                    (LocalVariables|SetNewEnLoc (Math|Vector|MakeVector (Math|Conversions|ToFloat(Integer) (.GridLocationX (Default|WorldtoGridCoordinates (LocalVariables|GetTheGrid) (Transformation|GetActorLocation (Utilities|Array|Get(acopy) (LocalVariables|GetTargets)))))) (Math|Conversions|ToFloat(Integer) (.GridLocationY (Default|WorldtoGridCoordinates (LocalVariables|GetTheGrid) (Transformation|GetActorLocation (Utilities|Array|Get(acopy) (LocalVariables|GetTargets)))))) 0.0))
                    (Variables|/Game/BattleBotsContent/Grid/BP_GridCell.BP_GridCell_C|SetUnit _gridcell_2 0)
                    (Default|PlaceUnit (LocalVariables|GetTheGrid) 0 0 (LocalVariables|GetEnUnit))
                    (Default|PlaceUnit (LocalVariables|GetTheGrid) (Math|Float|Truncate (.X (Math|Vector|BreakVector (LocalVariables|GetNewTeamLoc)))) (Math|Float|Truncate (.Y (Math|Vector|BreakVector (LocalVariables|GetNewTeamLoc)))) (Utilities|Array|Get(acopy) (LocalVariables|GetTargets)))
                    (Default|PlaceUnit (LocalVariables|GetTheGrid) (Math|Float|Truncate (.X (Math|Vector|BreakVector (LocalVariables|GetNewEnLoc)))) (Math|Float|Truncate (.Y (Math|Vector|BreakVector (LocalVariables|GetNewEnLoc)))) (LocalVariables|GetEnUnit))
                    (return false))
                  (:Is%20Not%20Valid
                    _)))
              (:CastFailed
                _))))
        (:CastFailed
          _)))
    (:CastFailed
      _))
  (return false))