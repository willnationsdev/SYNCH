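; BP_EffectTurret is a skill effect that adds damage dealing to the first skill of the user who used the triggering skill.
; Apply fetches that user's skills and checks whether the first one has any stored skill updaters.
; If so, it constructs a BP_EffectDealDamage owned by that skill and appends it to its effects to apply.
; Apply always returns false.
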(fn `Apply`
  (params (Skill :type "/Game/BattleBotsContent/Skills/BP_Skill Object Reference"))
  (returns (` ` :type Boolean))
  (bind _skills (`/Game/BattleBotsContent/Skills/BPI_SkillUser.GetSkills` (`/Game/BattleBotsContent/Skills/BP_Skill.SourceSkillUser` Skill)))
  (bind _item (`KismetArrayLibrary.Array_Get` _skills))
  (if (> (`KismetArrayLibrary.Array_Length` (`/Game/BattleBotsContent/Skills/BP_Skill.StoredSkillUpdaters` _item)) 0)
    (bind _returnvalue (`|GenericCreateObject` "/Game/BattleBotsContent/Skills/Effects/BP_EffectDealDamage.BP_EffectDealDamage_C" _item (`self.GameMode`)))
    (`KismetArrayLibrary.Array_Add` (`/Game/BattleBotsContent/Skills/BP_Skill.SkillEffectsToApply` _item) _returnvalue))
  (return false))