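; BP_EffectHeal is a skill effect that changes the current health of a skill's targets by the skill's Intensity attribute.
; Apply gathers the skill's user targets, filters them to valid ones, then applies DeltaHealth to each in turn.
; A target left at zero health or below is destroyed, and Apply returns that result immediately, skipping remaining targets; otherwise it returns false.
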(fn Apply
  (params (Skill :type BP%20Skill%20Object%20Reference))
  (bind _output_get (LocalVariables|SetTheSkill Skill))
  ;[1 1 1] For each target to be affected...
  (bind _targetskillusers (CallFunction|GetSkillUserTargets _output_get))
  (bind _filteredskillusers (CallFunction|FilterbyValidTarget _targetskillusers (LocalVariables|GetTheSkill)))
  (for _array_element _filteredskillusers
    (CallFunction|DeltaHealth _array_element (.Intensity (Utilities|Struct|BreakBPS_SkillAttributes (Variables|/Game/BattleBotsContent/Skills/BP_Skill.BP_Skill_C|GetSkillAttributes (LocalVariables|GetTheSkill)))))
    (bind _stats (Default|GetStats _array_element))
    ;[1 1 1] If the target's health has reached a "death" state, destroy the skill user.
    (if (<= (.CurrentHealth (Utilities|Struct|BreakBPS_Stats _stats)) 0)
      (bind __ (Default|DestroySkillUser _array_element))
      (return __)))
  (return false))