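; Skill effect that spawns an object, tar going by the asset name, for each target of a skill.
; Each spawn sits at the target unit's X/Y with Z at zero, or at the skill's target grid coordinates, used unscaled, if the target is no valid unit.
; The source unit's interact component performs the spawn, and Apply always returns true, stopping early when the source is not a unit.
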(fn Apply
  (params (Skill :type BP%20Skill%20Object%20Reference))
  (bind _targetskillusers (CallFunction|GetSkillUserTargets Skill))
  (for _array_element _targetskillusers
    (bind _asbp_unit (Utilities|Casting|CastToBP_Unit _array_element)
      (:then
        (Utilities|IsValid _asbp_unit
          (:Is%20Valid
            (LocalVariables|SetlocationToSpawn (Math|Vector|MakeVector (.X (Math|Vector|BreakVector (Transformation|GetActorLocation _asbp_unit))) (.Y (Math|Vector|BreakVector (Transformation|GetActorLocation _asbp_unit))) 0.0)))
          (:Is%20Not%20Valid
            (LocalVariables|SetlocationToSpawn (Math|Vector|MakeVector (Math|Conversions|ToFloat(Integer) (Variables|/Game/BattleBotsContent/Skills/BP_Skill.BP_Skill_C|GetTargetGridLocationX Skill)) (Math|Conversions|ToFloat(Integer) (Variables|/Game/BattleBotsContent/Skills/BP_Skill.BP_Skill_C|GetTargetGridLocationY Skill)) 0.0) :!label _label))))
      (:CastFailed
        (goto _label)))
    (bind _asbp_unit_2 (Utilities|Casting|CastToBP_Unit (Variables|/Game/BattleBotsContent/Skills/BP_Skill.BP_Skill_C|GetSourceSkillUser Skill))
      (:then
        (Default|Spawn (Variables|/Game/BattleBotsContent/Units/BP_Unit.BP_Unit_C|GetBP_UnitInteract_Component _asbp_unit_2) (LocalVariables|GetlocationToSpawn) "NewEnumerator4"))
      (:CastFailed
        (return true))))
  (return true))