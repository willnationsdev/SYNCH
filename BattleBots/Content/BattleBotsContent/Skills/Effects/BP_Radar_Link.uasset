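; BP_Radar_Link is a skill effect that hands stored skill updaters from the using unit to its target.
; Apply casts the skill's source user to BP_Unit, then appends the updaters stored on its first slotted skill to the first skill of the first target.
; It then clears the source skill's updater list, making this a move rather than a copy, and returns false.
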(fn `Apply`
  (params (Skill :type "/Game/BattleBotsContent/Skills/BP_Skill Object Reference"))
  (returns (` ` :type Boolean))
  (bind _targetskillusers (`self.GetSkillUserTargets` Skill))
  (bind _asbp_unit (cast `/Game/BattleBotsContent/Units/BP_Unit` (`/Game/BattleBotsContent/Skills/BP_Skill.SourceSkillUser` Skill))
    (:`then`
      (bind _skills (`/Game/BattleBotsContent/Skills/BPI_SkillUser.GetSkills` (`KismetArrayLibrary.Array_Get` _targetskillusers)))
      (bind _storedskillupdaters (`/Game/BattleBotsContent/Skills/BP_Skill.StoredSkillUpdaters` (`KismetArrayLibrary.Array_Get` (`/Game/BattleBotsContent/Units/BP_UnitComponent.SlottedSkills` (`/Game/BattleBotsContent/Units/BP_Unit.UnitComponent` _asbp_unit)))))
      (for _array_element _storedskillupdaters
        (`KismetArrayLibrary.Array_Add` (`/Game/BattleBotsContent/Skills/BP_Skill.StoredSkillUpdaters` (`KismetArrayLibrary.Array_Get` _skills)) _array_element)))
    (:`CastFailed`
      _))
  (`KismetArrayLibrary.Array_Clear` _storedskillupdaters)
  (return false))