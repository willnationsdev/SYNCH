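; Skill effect that displaces each targeted unit along the grid, using the skill user's position as the source of the force.
; Propel turns source and target locations into a short series of offsets, which are tested in order against the game mode's grid manager.
; Each unit is placed at the last empty cell before the first blocked one, or at its own cell if the first step is blocked.
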(fn Apply
  (params (Skill :type BP%20Skill%20Object%20Reference))
  (bind _asbpi_grid_managing_game_mode (Utilities|Casting|CastToBPI_GridManagingGameMode (Variables|Default|GetGameMode))
    (:then
      (bind _gridmanager (Default|GetGridManager _asbpi_grid_managing_game_mode))
      (LocalVariables|SetTheGrid _gridmanager)
      (bind _targetskillusers (CallFunction|GetSkillUserTargets Skill))
      (if (Utilities|IsValid (Utilities|ToObject(Interface) (Variables|/Game/BattleBotsContent/Skills/BP_Skill.BP_Skill_C|GetTargetSkillUser Skill)))
        _
        (else
          _))
      ;[1 1 1] Determine where we are coming from in terms of the "source" of the blast
      (bind _worldlocation (Default|GetWorldLocation (Variables|/Game/BattleBotsContent/Skills/BP_Skill.BP_Skill_C|GetSourceSkillUser Skill)))
      (LocalVariables|SetSourceVector _worldlocation)
      (for _array_element _targetskillusers
        (bind _worldlocation_2 (Default|GetWorldLocation _array_element))
        (LocalVariables|SetFinalLocation _worldlocation_2)
        (bind _propellantvectors (CallFunction|Propel (LocalVariables|GetSourceVector) _worldlocation_2 2))
        (bind _array_element_2 (Utilities|Array|ForEachLoopwithBreak _propellantvectors :!label _label)
          (:LoopBody
            (bind _isempty (Default|GridCellIsEmpty (LocalVariables|GetTheGrid) (.GridLocationX (Default|WorldtoGridCoordinates (LocalVariables|GetTheGrid) (+ _worldlocation_2 _array_element_2))) (.GridLocationY (Default|WorldtoGridCoordinates (LocalVariables|GetTheGrid) (+ _worldlocation_2 _array_element_2)))))
            (if _isempty
              (LocalVariables|SetFinalLocation (+ _worldlocation_2 _array_element_2))
              (else
                (goto _label Break))))
          (:Completed
            (bind _asbp_unit (Utilities|Casting|CastToBP_Unit _array_element))
            (Default|PlaceUnit (LocalVariables|GetTheGrid) (.GridLocationX (Default|WorldtoGridCoordinates (LocalVariables|GetTheGrid) (LocalVariables|GetFinalLocation))) (.GridLocationY (Default|WorldtoGridCoordinates (LocalVariables|GetTheGrid) (LocalVariables|GetFinalLocation))) _asbp_unit))))
      (return true))
    (:CastFailed
      (return false))))