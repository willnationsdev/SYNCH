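; Bull Rush skill effect that charges the caster across the battle grid toward the target, knocking back the first unit in its path.
; Apply steps cell by cell up to the skill's Intensity, stopping the caster before the first occupied cell.
; Leftover distance pushes the hit unit onward until blocked, and the grid manager places both units.
; It then sets that unit as TargetAlso on the effects of the caster's first slotted skill.
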(fn Apply
  (params (Skill :type BP%20Skill%20Object%20Reference))
  (bind _sourceskilluser (Variables|/Game/BattleBotsContent/Skills/BP_Skill.BP_Skill_C|GetSourceSkillUser Skill))
  (LocalVariables|SetHitUnit 0)
  (bind _worldlocation (Default|GetWorldLocation _sourceskilluser))
  (LocalVariables|SetplayerLocation _worldlocation)
  (bind _asbp_unit (Utilities|Casting|CastToBP_Unit _sourceskilluser)
    (:then
      (LocalVariables|SetCaster _asbp_unit)
      (LocalVariables|SetendLocation (Math|Vector|MakeVector (Math|Conversions|ToFloat(Integer) (Variables|/Game/BattleBotsContent/Skills/BP_Skill.BP_Skill_C|GetTargetGridLocationX Skill)) (Math|Conversions|ToFloat(Integer) (Variables|/Game/BattleBotsContent/Skills/BP_Skill.BP_Skill_C|GetTargetGridLocationY Skill)) 5e+01))
      (LocalVariables|SetDirection (Class|KismetMathLibrary|GetDirectionVector (LocalVariables|GetplayerLocation) (LocalVariables|GetendLocation)))
      (LocalVariables|SetDistance (.Intensity (Utilities|Struct|BreakBPS_SkillAttributes (Variables|/Game/BattleBotsContent/Skills/BP_Skill.BP_Skill_C|GetSkillAttributes Skill))))
      (Utilities|FlowControl|Sequence
        (:then_0
          (bind _asbpi_grid_managing_game_mode (Utilities|Casting|CastToBPI_GridManagingGameMode (Variables|Default|GetGameMode)))
          (bind _gridmanager (Default|GetGridManager _asbpi_grid_managing_game_mode))
          (LocalVariables|SetTheGrid _gridmanager))
        (:then_1
          (bind _index (Utilities|FlowControl|ForLoopwithBreak 1 (LocalVariables|GetDistance) :!label _label)
            (:LoopBody
              (bind _isempty (Default|GridCellIsEmpty (LocalVariables|GetTheGrid) (.GridLocationX (Default|WorldtoGridCoordinates (LocalVariables|GetTheGrid) (+ (LocalVariables|GetplayerLocation) (* (LocalVariables|GetDirection) (* _index 100))))) (.GridLocationY (Default|WorldtoGridCoordinates (LocalVariables|GetTheGrid) (+ (LocalVariables|GetplayerLocation) (* (LocalVariables|GetDirection) (* _index 100)))))))
              (if _isempty
                (LocalVariables|SetFinalPoint (+ (LocalVariables|GetplayerLocation) (* (LocalVariables|GetDirection) (* _index 100))))
                (else
                  (bind _gridcell (Default|GetGridCellfromCoordinates (LocalVariables|GetTheGrid) (.GridLocationX (Default|WorldtoGridCoordinates (LocalVariables|GetTheGrid) (+ (LocalVariables|GetplayerLocation) (* (LocalVariables|GetDirection) (* _index 100))))) (.GridLocationY (Default|WorldtoGridCoordinates (LocalVariables|GetTheGrid) (+ (LocalVariables|GetplayerLocation) (* (LocalVariables|GetDirection) (* _index 100)))))))
                  (LocalVariables|SetHitUnit (Variables|/Game/BattleBotsContent/Grid/BP_GridCell.BP_GridCell_C|GetUnit _gridcell))
                  (LocalVariables|SetLastIndex _index)
                  (goto _label Break))))))
        (:then_2
          (if (LocalVariables|GetfirstTimeOnly)
            (LocalVariables|SetfirstTimeOnly false)
            (if (Math|Vector|Equal(Vector) "-1.000000,-1.000000,-1.000000" (LocalVariables|GetFinalPoint) 0.0001)
              (LocalVariables|SetFinalPoint (LocalVariables|GetplayerLocation)))
            (bind _index_2 (Utilities|FlowControl|ForLoopwithBreak 2 (+ (- (LocalVariables|GetDistance) (LocalVariables|GetLastIndex)) 1) :!label _label_2)
              (:LoopBody
                (bind _isempty_2 (Default|GridCellIsEmpty (LocalVariables|GetTheGrid) (.GridLocationX (Default|WorldtoGridCoordinates (LocalVariables|GetTheGrid) (+ (LocalVariables|GetFinalPoint) (* (LocalVariables|GetDirection) (* _index_2 100))))) (.GridLocationY (Default|WorldtoGridCoordinates (LocalVariables|GetTheGrid) (+ (LocalVariables|GetFinalPoint) (* (LocalVariables|GetDirection) (* _index_2 100)))))))
                (if _isempty_2
                  (LocalVariables|SetFinalPointHit (+ (LocalVariables|GetFinalPoint) (* (LocalVariables|GetDirection) (* _index_2 100))))
                  (else
                    (goto _label_2 Break)))))))
        (:then_3
          (if (Math|Vector|NotEqual(Vector) "-1.000000,-1.000000,-1.000000" (LocalVariables|GetFinalPointHit) 0.0001)
            (Default|PlaceUnit (LocalVariables|GetTheGrid) (.GridLocationX (Default|WorldtoGridCoordinates (LocalVariables|GetTheGrid) (LocalVariables|GetFinalPointHit))) (.GridLocationY (Default|WorldtoGridCoordinates (LocalVariables|GetTheGrid) (LocalVariables|GetFinalPointHit))) (LocalVariables|GetHitUnit))))
        (:then_4
          (goto _label))
        (:then_6
          (Default|PlaceUnit (LocalVariables|GetTheGrid) (.GridLocationX (Default|WorldtoGridCoordinates (LocalVariables|GetTheGrid) (LocalVariables|GetFinalPoint))) (.GridLocationY (Default|WorldtoGridCoordinates (LocalVariables|GetTheGrid) (LocalVariables|GetFinalPoint))) (LocalVariables|GetCaster)))
        (:then_7
          (Utilities|Array|Clear (Variables|Default|GetTargetAlso))
          (for _array_element (Variables|/Game/BattleBotsContent/Skills/BP_Skill.BP_Skill_C|GetSkillEffectsToApply (Utilities|Array|Get(acopy) (Variables|/Game/BattleBotsContent/Units/BP_UnitComponent.BP_UnitComponent_C|GetSlottedSkills (Variables|/Game/BattleBotsContent/Units/BP_Unit.BP_Unit_C|GetUnitComponent (LocalVariables|GetCaster)))))
            (Utilities|Array|Clear (Variables|/Game/BattleBotsContent/Skills/BP_SkillEffect.BP_SkillEffect_C|GetTargetAlso _array_element))
            (Utilities|IsValid (LocalVariables|GetHitUnit)
              (:Is%20Valid
                (if (!= (LocalVariables|GetHitUnit) (LocalVariables|GetCaster))
                  (Utilities|Array|Add (Variables|/Game/BattleBotsContent/Skills/BP_SkillEffect.BP_SkillEffect_C|GetTargetAlso _array_element) (LocalVariables|GetHitUnit))))))
          (return false))))
    (:CastFailed
      (return false))))