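; Skill effect for the super acid activation, spawning objects (presumably acid) on the battle grid around the casting unit.
; Apply first spawns at each TargetAlso location stored in the caster's first slotted skill effect, then clears that list.
; It then checks the eight surrounding cells through the grid manager, spawning via the unit's interact component in any cell not occupied by the caster.
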(fn Apply
  (params (Skill :type BP%20Skill%20Object%20Reference))
  (bind _sourceskilluser (Variables|/Game/BattleBotsContent/Skills/BP_Skill.BP_Skill_C|GetSourceSkillUser Skill))
  (bind _asbpi_grid_managing_game_mode (Utilities|Casting|CastToBPI_GridManagingGameMode (Variables|Default|GetGameMode))
    (:then
      (bind _gridmanager (Default|GetGridManager _asbpi_grid_managing_game_mode))
      (LocalVariables|SetTheGrid _gridmanager)
      (bind _asbp_unit (Utilities|Casting|CastToBP_Unit _sourceskilluser)
        (:then
          (for _array_element (Variables|/Game/BattleBotsContent/Skills/BP_SkillEffect.BP_SkillEffect_C|GetTargetAlso (Utilities|Array|Get(acopy) (Variables|/Game/BattleBotsContent/Skills/BP_Skill.BP_Skill_C|GetSkillEffectsToApply (Utilities|Array|Get(acopy) (Variables|/Game/BattleBotsContent/Units/BP_UnitComponent.BP_UnitComponent_C|GetSlottedSkills (Variables|/Game/BattleBotsContent/Units/BP_Unit.BP_Unit_C|GetUnitComponent _asbp_unit))))))
            (bind _worldlocation (Default|GetWorldLocation _array_element))
            (Default|Spawn (Variables|/Game/BattleBotsContent/Units/BP_Unit.BP_Unit_C|GetBP_UnitInteract_Component _asbp_unit) (Math|Vector|MakeVector (.X (Math|Vector|BreakVector _worldlocation)) (.Y (Math|Vector|BreakVector _worldlocation)) 0.0) "NewEnumerator0"))
          (Utilities|Array|Clear (Variables|/Game/BattleBotsContent/Skills/BP_SkillEffect.BP_SkillEffect_C|GetTargetAlso (Utilities|Array|Get(acopy) (Variables|/Game/BattleBotsContent/Skills/BP_Skill.BP_Skill_C|GetSkillEffectsToApply (Utilities|Array|Get(acopy) (Variables|/Game/BattleBotsContent/Units/BP_UnitComponent.BP_UnitComponent_C|GetSlottedSkills (Variables|/Game/BattleBotsContent/Units/BP_Unit.BP_Unit_C|GetUnitComponent _asbp_unit)))))))
          (bind _worldlocation_2 (Default|GetWorldLocation _sourceskilluser))
          (Utilities|FlowControl|Sequence
            (:then_0
              (LocalVariables|SettempVector (+ _worldlocation_2 "100.000000, 0, 0")))
            (:then_1
              (LocalVariables|SettempVector (+ _worldlocation_2 "0,100.000000, 0")))
            (:then_2
              (LocalVariables|SettempVector (+ _worldlocation_2 "-100.000000, 0, 0")))
            (:then_3
              (LocalVariables|SettempVector (+ _worldlocation_2 "0,-100.000000, 0")))
            (:then_4
              (LocalVariables|SettempVector (+ _worldlocation_2 "100.000000,100.000000, 0")))
            (:then_5
              (LocalVariables|SettempVector (+ _worldlocation_2 "100.000000,-100.000000, 0")))
            (:then_6
              (LocalVariables|SettempVector (+ _worldlocation_2 "-100.000000,100.000000, 0")))
            (:then_7
              (LocalVariables|SettempVector (+ _worldlocation_2 "-100.000000,-100.000000, 0"))))
          (bind _gridcell (Default|GetGridCellfromCoordinates (LocalVariables|GetTheGrid) (.GridLocationX (Default|WorldtoGridCoordinates (LocalVariables|GetTheGrid) (LocalVariables|GettempVector))) (.GridLocationY (Default|WorldtoGridCoordinates (LocalVariables|GetTheGrid) (LocalVariables|GettempVector)))))
          (if (!= _asbp_unit (Variables|/Game/BattleBotsContent/Grid/BP_GridCell.BP_GridCell_C|GetUnit _gridcell))
            (Default|Spawn (Variables|/Game/BattleBotsContent/Units/BP_Unit.BP_Unit_C|GetBP_UnitInteract_Component _asbp_unit) (Math|Vector|MakeVector (* (.GridLocationX (Default|WorldtoGridCoordinates (LocalVariables|GetTheGrid) (LocalVariables|GettempVector))) 1e+02) (* (.GridLocationY (Default|WorldtoGridCoordinates (LocalVariables|GetTheGrid) (LocalVariables|GettempVector))) 1e+02) 5.0) "NewEnumerator0")))
        (:CastFailed
          (return false))))
    (:CastFailed
      (return false))))