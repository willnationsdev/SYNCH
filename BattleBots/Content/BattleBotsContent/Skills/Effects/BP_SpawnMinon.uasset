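; Skill effect that spawns minions on grid cells in a line from the caster toward the target, out to the first slotted skill's range, one step further off-axis.
; Blocked cells fall back to searching their eight neighbours, stopping after the first successful fallback spawn.
; It then copies the caster's stored skill updaters to units on the spawned cells and clears the caster's updaters and pending skill effects.
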(fn Apply
  (params (Skill :type BP%20Skill%20Object%20Reference))
  (bind _sourceskilluser (Variables|/Game/BattleBotsContent/Skills/BP_Skill.BP_Skill_C|GetSourceSkillUser Skill))
  (bind _xy (LocalVariables|GetXY))
  (bind _worldlocation (Default|GetWorldLocation _sourceskilluser))
  (bind _output_get (LocalVariables|SetcharacterLocation _worldlocation))
  (LocalVariables|SetEndLocation (Math|Vector|MakeVector (Math|Conversions|ToFloat(Integer) (Variables|/Game/BattleBotsContent/Skills/BP_Skill.BP_Skill_C|GetTargetGridLocationX Skill)) (Math|Conversions|ToFloat(Integer) (Variables|/Game/BattleBotsContent/Skills/BP_Skill.BP_Skill_C|GetTargetGridLocationY Skill)) (.Z (Math|Vector|BreakVector _output_get))))
  (bind _asbp_unit (Utilities|Casting|CastToBP_Unit _sourceskilluser)
    (:then
      (bind _asbpi_grid_managing_game_mode (Utilities|Casting|CastToBPI_GridManagingGameMode (Variables|Default|GetGameMode))
        (:then
          (bind _gridmanager (Default|GetGridManager _asbpi_grid_managing_game_mode))
          (LocalVariables|SettheGrid _gridmanager)
          (if (or (== (Math|Float|Absolute(Float) (.X (Math|Vector|BreakVector (Class|KismetMathLibrary|GetDirectionVector (LocalVariables|GetcharacterLocation) (LocalVariables|GetEndLocation))))) 1.0) (== (Math|Float|Absolute(Float) (.Y (Math|Vector|BreakVector (Class|KismetMathLibrary|GetDirectionVector (LocalVariables|GetcharacterLocation) (LocalVariables|GetEndLocation))))) 1.0))
            (LocalVariables|Setinc 0)
            (else
              (LocalVariables|Setinc 1)))
          (for _index (range 1 (+ (.Range (Utilities|Struct|BreakBPS_SkillAttributes (Variables|/Game/BattleBotsContent/Skills/BP_Skill.BP_Skill_C|GetSkillAttributes (Utilities|Array|Get(acopy) (Variables|/Game/BattleBotsContent/Units/BP_UnitComponent.BP_UnitComponent_C|GetSlottedSkills (Variables|/Game/BattleBotsContent/Units/BP_Unit.BP_Unit_C|GetUnitComponent _asbp_unit)))))) (LocalVariables|Getinc)))
            (bind _isempty (Default|GridCellIsEmpty (LocalVariables|GettheGrid) (.GridLocationX (Default|WorldtoGridCoordinates (LocalVariables|GetTheGrid) (Math|Vector|MakeVector (+ (.X (Math|Vector|BreakVector (LocalVariables|GetcharacterLocation))) (.X (Math|Vector|BreakVector (* (Class|KismetMathLibrary|GetDirectionVector (LocalVariables|GetcharacterLocation) (LocalVariables|GetEndLocation)) (* _index 100))))) (+ (.Y (Math|Vector|BreakVector (LocalVariables|GetcharacterLocation))) (.Y (Math|Vector|BreakVector (* (Class|KismetMathLibrary|GetDirectionVector (LocalVariables|GetcharacterLocation) (LocalVariables|GetEndLocation)) (* _index 100))))) 0.0))) (.GridLocationY (Default|WorldtoGridCoordinates (LocalVariables|GetTheGrid) (Math|Vector|MakeVector (+ (.X (Math|Vector|BreakVector (LocalVariables|GetcharacterLocation))) (.X (Math|Vector|BreakVector (* (Class|KismetMathLibrary|GetDirectionVector (LocalVariables|GetcharacterLocation) (LocalVariables|GetEndLocation)) (* _index 100))))) (+ (.Y (Math|Vector|BreakVector (LocalVariables|GetcharacterLocation))) (.Y (Math|Vector|BreakVector (* (Class|KismetMathLibrary|GetDirectionVector (LocalVariables|GetcharacterLocation) (LocalVariables|GetEndLocation)) (* _index 100))))) 0.0)))))
            (if _isempty
              (Utilities|Array|Add (LocalVariables|GetSuccessSpawn) (Math|Vector|MakeVector (Math|Conversions|ToFloat(Integer) (.GridLocationX (Default|WorldtoGridCoordinates (LocalVariables|GetTheGrid) (Math|Vector|MakeVector (+ (.X (Math|Vector|BreakVector (LocalVariables|GetcharacterLocation))) (.X (Math|Vector|BreakVector (* (Class|KismetMathLibrary|GetDirectionVector (LocalVariables|GetcharacterLocation) (LocalVariables|GetEndLocation)) (* _index 100))))) (+ (.Y (Math|Vector|BreakVector (LocalVariables|GetcharacterLocation))) (.Y (Math|Vector|BreakVector (* (Class|KismetMathLibrary|GetDirectionVector (LocalVariables|GetcharacterLocation) (LocalVariables|GetEndLocation)) (* _index 100))))) 0.0)))) (Math|Conversions|ToFloat(Integer) (.GridLocationY (Default|WorldtoGridCoordinates (LocalVariables|GetTheGrid) (Math|Vector|MakeVector (+ (.X (Math|Vector|BreakVector (LocalVariables|GetcharacterLocation))) (.X (Math|Vector|BreakVector (* (Class|KismetMathLibrary|GetDirectionVector (LocalVariables|GetcharacterLocation) (LocalVariables|GetEndLocation)) (* _index 100))))) (+ (.Y (Math|Vector|BreakVector (LocalVariables|GetcharacterLocation))) (.Y (Math|Vector|BreakVector (* (Class|KismetMathLibrary|GetDirectionVector (LocalVariables|GetcharacterLocation) (LocalVariables|GetEndLocation)) (* _index 100))))) 0.0)))) 0.0))
              (Default|Spawn (Variables|/Game/BattleBotsContent/Units/BP_Unit.BP_Unit_C|GetBP_UnitInteract_Component _asbp_unit) (Math|Vector|MakeVector (* (.GridLocationX (Default|WorldtoGridCoordinates (LocalVariables|GetTheGrid) (Math|Vector|MakeVector (+ (.X (Math|Vector|BreakVector (LocalVariables|GetcharacterLocation))) (.X (Math|Vector|BreakVector (* (Class|KismetMathLibrary|GetDirectionVector (LocalVariables|GetcharacterLocation) (LocalVariables|GetEndLocation)) (* _index 100))))) (+ (.Y (Math|Vector|BreakVector (LocalVariables|GetcharacterLocation))) (.Y (Math|Vector|BreakVector (* (Class|KismetMathLibrary|GetDirectionVector (LocalVariables|GetcharacterLocation) (LocalVariables|GetEndLocation)) (* _index 100))))) 0.0))) 1e+02) (* (.GridLocationY (Default|WorldtoGridCoordinates (LocalVariables|GetTheGrid) (Math|Vector|MakeVector (+ (.X (Math|Vector|BreakVector (LocalVariables|GetcharacterLocation))) (.X (Math|Vector|BreakVector (* (Class|KismetMathLibrary|GetDirectionVector (LocalVariables|GetcharacterLocation) (LocalVariables|GetEndLocation)) (* _index 100))))) (+ (.Y (Math|Vector|BreakVector (LocalVariables|GetcharacterLocation))) (.Y (Math|Vector|BreakVector (* (Class|KismetMathLibrary|GetDirectionVector (LocalVariables|GetcharacterLocation) (LocalVariables|GetEndLocation)) (* _index 100))))) 0.0))) 1e+02) 0.0) "NewEnumerator2")
              (else
                (Utilities|Array|Add _xy (Math|Vector|MakeVector (Math|Conversions|ToFloat(Integer) (.GridLocationX (Default|WorldtoGridCoordinates (LocalVariables|GetTheGrid) (Math|Vector|MakeVector (+ (.X (Math|Vector|BreakVector (LocalVariables|GetcharacterLocation))) (.X (Math|Vector|BreakVector (* (Class|KismetMathLibrary|GetDirectionVector (LocalVariables|GetcharacterLocation) (LocalVariables|GetEndLocation)) (* _index 100))))) (+ (.Y (Math|Vector|BreakVector (LocalVariables|GetcharacterLocation))) (.Y (Math|Vector|BreakVector (* (Class|KismetMathLibrary|GetDirectionVector (LocalVariables|GetcharacterLocation) (LocalVariables|GetEndLocation)) (* _index 100))))) 0.0)))) (Math|Conversions|ToFloat(Integer) (.GridLocationY (Default|WorldtoGridCoordinates (LocalVariables|GetTheGrid) (Math|Vector|MakeVector (+ (.X (Math|Vector|BreakVector (LocalVariables|GetcharacterLocation))) (.X (Math|Vector|BreakVector (* (Class|KismetMathLibrary|GetDirectionVector (LocalVariables|GetcharacterLocation) (LocalVariables|GetEndLocation)) (* _index 100))))) (+ (.Y (Math|Vector|BreakVector (LocalVariables|GetcharacterLocation))) (.Y (Math|Vector|BreakVector (* (Class|KismetMathLibrary|GetDirectionVector (LocalVariables|GetcharacterLocation) (LocalVariables|GetEndLocation)) (* _index 100))))) 0.0)))) 0.0))
                (for _array_element (LocalVariables|GetSuccessSpawn)
                  (Utilities|Array|RemoveItem _xy _array_element)))))
          (for _array_element_2 (LocalVariables|GetXY)
            (Utilities|FlowControl|Sequence
              (:then_0
                (LocalVariables|SettempVec (+ _array_element_2 "1.000000, 0, 0")))
              (:then_1
                (LocalVariables|SettempVec (+ _array_element_2 "0,1.000000, 0")))
              (:then_2
                (LocalVariables|SettempVec (+ _array_element_2 "-1.000000, 0, 0")))
              (:then_3
                (LocalVariables|SettempVec (+ _array_element_2 "0,-1.000000, 0")))
              (:then_4
                (LocalVariables|SettempVec (+ _array_element_2 "1.000000,1.000000, 0")))
              (:then_5
                (LocalVariables|SettempVec (+ _array_element_2 "1.000000,-1.000000, 0")))
              (:then_6
                (LocalVariables|SettempVec (+ _array_element_2 "-1.000000,1.000000, 0")))
              (:then_7
                (LocalVariables|SettempVec (+ _array_element_2 "-1.000000,-1.000000, 0"))))
            (bind _isempty_2 (Default|GridCellIsEmpty (LocalVariables|GettheGrid) (Math|Float|Truncate (.X (Math|Vector|BreakVector (LocalVariables|GettempVec)))) (Math|Float|Truncate (.Y (Math|Vector|BreakVector (LocalVariables|GettempVec))))))
            (if _isempty_2
              (Default|Spawn (Variables|/Game/BattleBotsContent/Units/BP_Unit.BP_Unit_C|GetBP_UnitInteract_Component _asbp_unit) (* (LocalVariables|GettempVec) 1e+02) "NewEnumerator2")
              (Utilities|Array|Add (LocalVariables|GetSuccessSpawn) (LocalVariables|GettempVec))
              (Utilities|FlowControl|Sequence
                (:then_0
                  (for _array_element_3 (LocalVariables|GetSuccessSpawn)
                    (bind _gridcell (Default|GetGridCellfromCoordinates (LocalVariables|GettheGrid) (Math|Float|Truncate (.X (Math|Vector|BreakVector _array_element_3))) (Math|Float|Truncate (.Y (Math|Vector|BreakVector _array_element_3)))))
                    (Utilities|IsValid (Variables|/Game/BattleBotsContent/Grid/BP_GridCell.BP_GridCell_C|GetUnit _gridcell)
                      (:Is%20Valid
                        (for _array_element_4 (Variables|/Game/BattleBotsContent/Skills/BP_Skill.BP_Skill_C|GetStoredSkillUpdaters (Utilities|Array|Get(acopy) (Variables|/Game/BattleBotsContent/Units/BP_UnitComponent.BP_UnitComponent_C|GetSlottedSkills (Variables|/Game/BattleBotsContent/Units/BP_Unit.BP_Unit_C|GetUnitComponent _asbp_unit))))
                          (Utilities|Array|Add (Variables|/Game/BattleBotsContent/Skills/BP_Skill.BP_Skill_C|GetStoredSkillUpdaters (Utilities|Array|Get(acopy) (Variables|/Game/BattleBotsContent/Units/BP_UnitComponent.BP_UnitComponent_C|GetSlottedSkills (Variables|/Game/BattleBotsContent/Units/BP_Unit.BP_Unit_C|GetUnitComponent (Variables|/Game/BattleBotsContent/Grid/BP_GridCell.BP_GridCell_C|GetUnit _gridcell))))) _array_element_4))))))
                (:then_1
                  (Utilities|Array|Clear (Variables|/Game/BattleBotsContent/Skills/BP_Skill.BP_Skill_C|GetSkillEffectsToApply (Utilities|Array|Get(acopy) (Variables|/Game/BattleBotsContent/Units/BP_UnitComponent.BP_UnitComponent_C|GetSlottedSkills (Variables|/Game/BattleBotsContent/Units/BP_Unit.BP_Unit_C|GetUnitComponent _asbp_unit)))))
                  (Utilities|Array|Clear (Variables|/Game/BattleBotsContent/Skills/BP_Skill.BP_Skill_C|GetStoredSkillUpdaters (Utilities|Array|Get(acopy) (Variables|/Game/BattleBotsContent/Units/BP_UnitComponent.BP_UnitComponent_C|GetSlottedSkills (Variables|/Game/BattleBotsContent/Units/BP_Unit.BP_Unit_C|GetUnitComponent _asbp_unit)))))
                  (return true)))))
          (Utilities|FlowControl|Sequence
            (:then_0
              (for _array_element_5 (LocalVariables|GetSuccessSpawn)
                (bind _gridcell_2 (Default|GetGridCellfromCoordinates (LocalVariables|GettheGrid) (Math|Float|Truncate (.X (Math|Vector|BreakVector _array_element_5))) (Math|Float|Truncate (.Y (Math|Vector|BreakVector _array_element_5)))))
                (Utilities|IsValid (Variables|/Game/BattleBotsContent/Grid/BP_GridCell.BP_GridCell_C|GetUnit _gridcell_2)
                  (:Is%20Valid
                    (for _array_element_6 (Variables|/Game/BattleBotsContent/Skills/BP_Skill.BP_Skill_C|GetStoredSkillUpdaters (Utilities|Array|Get(acopy) (Variables|/Game/BattleBotsContent/Units/BP_UnitComponent.BP_UnitComponent_C|GetSlottedSkills (Variables|/Game/BattleBotsContent/Units/BP_Unit.BP_Unit_C|GetUnitComponent _asbp_unit))))
                      (Utilities|Array|Add (Variables|/Game/BattleBotsContent/Skills/BP_Skill.BP_Skill_C|GetStoredSkillUpdaters (Utilities|Array|Get(acopy) (Variables|/Game/BattleBotsContent/Units/BP_UnitComponent.BP_UnitComponent_C|GetSlottedSkills (Variables|/Game/BattleBotsContent/Units/BP_Unit.BP_Unit_C|GetUnitComponent (Variables|/Game/BattleBotsContent/Grid/BP_GridCell.BP_GridCell_C|GetUnit _gridcell_2))))) _array_element_6))))))
            (:then_1
              (Utilities|Array|Clear (Variables|/Game/BattleBotsContent/Skills/BP_Skill.BP_Skill_C|GetSkillEffectsToApply (Utilities|Array|Get(acopy) (Variables|/Game/BattleBotsContent/Units/BP_UnitComponent.BP_UnitComponent_C|GetSlottedSkills (Variables|/Game/BattleBotsContent/Units/BP_Unit.BP_Unit_C|GetUnitComponent _asbp_unit)))))
              (Utilities|Array|Clear (Variables|/Game/BattleBotsContent/Skills/BP_Skill.BP_Skill_C|GetStoredSkillUpdaters (Utilities|Array|Get(acopy) (Variables|/Game/BattleBotsContent/Units/BP_UnitComponent.BP_UnitComponent_C|GetSlottedSkills (Variables|/Game/BattleBotsContent/Units/BP_Unit.BP_Unit_C|GetUnitComponent _asbp_unit)))))
              (return true))))
        (:CastFailed
          (return false))))
    (:CastFailed
      (return false))))