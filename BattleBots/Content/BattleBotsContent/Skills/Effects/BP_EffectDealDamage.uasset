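; BP_EffectDealDamage is a skill effect that damages every valid target of the skill being applied.
; Apply filters the skill's targets, then lowers each one's health by the skill's Intensity, adjusted by TraceDamage for Traced units.
; Targets left at zero health or below are destroyed.
; It always returns false and never calls the parent Apply; a failed BP_Unit cast only logs that trace was skipped.
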(fn Apply
  (params (Skill :type BP%20Skill%20Object%20Reference))
  (bind _output_get (LocalVariables|SetTheSkill Skill))
  ;[1 1 1] For each target to be affected...
  (bind _targetskillusers (CallFunction|GetSkillUserTargets _output_get))
  (bind _filteredskillusers (CallFunction|FilterbyValidTarget _targetskillusers (LocalVariables|GetTheSkill)))
  (for _array_element _filteredskillusers
    (Variables|Default|SetHealthToDeltify (* (.Intensity (Utilities|Struct|BreakBPS_SkillAttributes (Variables|/Game/BattleBotsContent/Skills/BP_Skill.BP_Skill_C|GetSkillAttributes (LocalVariables|GetTheSkill)))) -1))
    ;[1 1 1] Check if traced. If so, add trace damage
    (bind _asbp_unit (Utilities|Casting|CastToBP_Unit (Utilities|ToObject(Interface) _array_element))
      (:then
        (if (Variables|/Game/BattleBotsContent/Units/BP_UnitComponent.BP_UnitComponent_C|GetTraced (Variables|/Game/BattleBotsContent/Units/BP_Unit.BP_Unit_C|GetUnitComponent _asbp_unit))
          (Variables|Default|SetHealthToDeltify (+ (Variables|Default|GetHealthToDeltify) (Variables|Default|GetTraceDamage)))))
      (:CastFailed
        (Development|PrintString (Utilities|ToObject(Interface) _array_element) "BP_EffectDealDamage::Apply: Error! Failed to cast target skill user to BP_Unit. TRACE NOT APPLIED")))
    (CallFunction|DeltaHealth _array_element (Variables|Default|GetHealthToDeltify))
    (bind _stats (Default|GetStats _array_element))
    ;[1 1 1] If the target's health has reached a "death" state, destroy the skill user.
    (if (<= (.CurrentHealth (Utilities|Struct|BreakBPS_Stats _stats)) 0)
      (Default|DestroySkillUser _array_element)))
  (return false))