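; Skill effect that picks a random enemy unit as an extra target for the caster's skill, presumably Super Acid.
; Apply gathers all units from the game mode, keeps those not on the caster's team, shuffles them and steps past units named "Minion".
; The chosen unit is appended to TargetAlso on the first effect of the caster's first slotted skill, and Apply always returns false.
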(fn Apply
  (params (Skill :type BP%20Skill%20Object%20Reference))
  (bind _shuffler (LocalVariables|Getshuffler))
  (bind _index (LocalVariables|Getindex))
  (bind _item (Utilities|Array|Get(acopy) _shuffler _index))
  (bind _asbp_battle_game_mode (Utilities|Casting|CastToBP_BattleGameMode (Variables|Default|GetGameMode))
    (:then
      (bind _allunits (Default|GetAllunits _asbp_battle_game_mode))
      (bind _asbp_unit (Utilities|Casting|CastToBP_Unit (Variables|/Game/BattleBotsContent/Skills/BP_Skill.BP_Skill_C|GetSourceSkillUser Skill))
        (:then
          (LocalVariables|SetCaster _asbp_unit)
          (for _array_element _allunits
            (if (Utilities|Enum|NotEqual(Enum) (Variables|/Game/BattleBotsContent/Units/BP_UnitTeamComponent.BP_UnitTeamComponent_C|GetTeam (Variables|/Game/BattleBotsContent/Units/BP_Unit.BP_Unit_C|GetBP_UnitTeamComponent (LocalVariables|GetCaster))) (Variables|/Game/BattleBotsContent/Units/BP_UnitTeamComponent.BP_UnitTeamComponent_C|GetTeam (Variables|/Game/BattleBotsContent/Units/BP_Unit.BP_Unit_C|GetBP_UnitTeamComponent _array_element)))
              (Utilities|Array|Add (LocalVariables|Getshuffler) _array_element)))
          (Utilities|Array|Shuffle _shuffler)
          (if (and (Utilities|Name|Equal(Name) (Variables|/Game/BattleBotsContent/Units/BP_UnitComponent.BP_UnitComponent_C|GetUnitName (Variables|/Game/BattleBotsContent/Units/BP_Unit.BP_Unit_C|GetUnitComponent _item)) "Minion") (< _index (Utilities|Array|Length _shuffler))) :!label _label
            (Math|Integer|IncrementInt (LocalVariables|Getindex)
              (:%20%20
                (goto _label)))
            (else
              (Utilities|Array|Add (Variables|/Game/BattleBotsContent/Skills/BP_SkillEffect.BP_SkillEffect_C|GetTargetAlso (Utilities|Array|Get(acopy) (Variables|/Game/BattleBotsContent/Skills/BP_Skill.BP_Skill_C|GetSkillEffectsToApply (Utilities|Array|Get(acopy) (Variables|/Game/BattleBotsContent/Units/BP_UnitComponent.BP_UnitComponent_C|GetSlottedSkills (Variables|/Game/BattleBotsContent/Units/BP_Unit.BP_Unit_C|GetUnitComponent (LocalVariables|GetCaster))))))) _item)
              (return false))))
        (:CastFailed
          _)))
    (:CastFailed
      _))
  (return false))