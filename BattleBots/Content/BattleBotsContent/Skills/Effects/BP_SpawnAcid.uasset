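; Skill effect that spawns a line of acid across grid cells from the casting unit toward the skill's target.
; It steps along the direction vector for the slot 0 skill's range plus one cell, or two when off-axis, spawning through the unit's interact component.
; It also rebuilds TargetAlso on that slot 0 skill's effects, rather than the passed skill's, with units found along the line.
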(fn Apply
  (params (Skill :type BP%20Skill%20Object%20Reference))
  (bind _sourceskilluser (Variables|/Game/BattleBotsContent/Skills/BP_Skill.BP_Skill_C|GetSourceSkillUser Skill))
  (bind _worldlocation (Default|GetWorldLocation _sourceskilluser))
  (LocalVariables|SetcharacterLocation _worldlocation)
  (LocalVariables|SetEndLocation (Math|Vector|MakeVector (Math|Conversions|ToFloat(Integer) (Variables|/Game/BattleBotsContent/Skills/BP_Skill.BP_Skill_C|GetTargetGridLocationX Skill)) (Math|Conversions|ToFloat(Integer) (Variables|/Game/BattleBotsContent/Skills/BP_Skill.BP_Skill_C|GetTargetGridLocationY Skill)) 5e+01))
  (bind _asbpi_grid_managing_game_mode (Utilities|Casting|CastToBPI_GridManagingGameMode (Variables|Default|GetGameMode))
    (:then
      (bind _gridmanager (Default|GetGridManager _asbpi_grid_managing_game_mode))
      (LocalVariables|SetTheGrid _gridmanager)
      (bind _asbp_unit (Utilities|Casting|CastToBP_Unit _sourceskilluser)
        (:then
          (for _array_element (Variables|/Game/BattleBotsContent/Skills/BP_Skill.BP_Skill_C|GetSkillEffectsToApply (Utilities|Array|Get(acopy) (Variables|/Game/BattleBotsContent/Units/BP_UnitComponent.BP_UnitComponent_C|GetSlottedSkills (Variables|/Game/BattleBotsContent/Units/BP_Unit.BP_Unit_C|GetUnitComponent _asbp_unit))))
            (Utilities|Array|Clear (Variables|/Game/BattleBotsContent/Skills/BP_SkillEffect.BP_SkillEffect_C|GetTargetAlso _array_element)))
          (bind _resultantskill (Default|GetResultSkill (Utilities|Array|Get(acopy) (Variables|/Game/BattleBotsContent/Units/BP_UnitComponent.BP_UnitComponent_C|GetSlottedSkills (Variables|/Game/BattleBotsContent/Units/BP_Unit.BP_Unit_C|GetUnitComponent _asbp_unit)))))
          (if (or (== (Math|Float|Absolute(Float) (.X (Math|Vector|BreakVector (Class|KismetMathLibrary|GetDirectionVector (LocalVariables|GetcharacterLocation) (LocalVariables|GetEndLocation))))) 1.0) (== (Math|Float|Absolute(Float) (.Y (Math|Vector|BreakVector (Class|KismetMathLibrary|GetDirectionVector (LocalVariables|GetcharacterLocation) (LocalVariables|GetEndLocation))))) 1.0))
            (LocalVariables|Setinc 1)
            (else
              (LocalVariables|Setinc 2)))
          (for _index (range 1 (+ (.Range (Utilities|Struct|BreakBPS_SkillAttributes (Variables|/Game/BattleBotsContent/Skills/BP_Skill.BP_Skill_C|GetSkillAttributes _resultantskill))) (LocalVariables|Getinc)))
            (bind _gridcell (Default|GetGridCellfromCoordinates (LocalVariables|GetTheGrid) (.GridLocationX (Default|WorldtoGridCoordinates (LocalVariables|GetTheGrid) (Math|Vector|MakeVector (+ (.X (Math|Vector|BreakVector (LocalVariables|GetcharacterLocation))) (.X (Math|Vector|BreakVector (* (Class|KismetMathLibrary|GetDirectionVector (LocalVariables|GetcharacterLocation) (LocalVariables|GetEndLocation)) (* _index 100))))) (+ (.Y (Math|Vector|BreakVector (LocalVariables|GetcharacterLocation))) (.Y (Math|Vector|BreakVector (* (Class|KismetMathLibrary|GetDirectionVector (LocalVariables|GetcharacterLocation) (LocalVariables|GetEndLocation)) (* _index 100))))) 0.0))) (.GridLocationY (Default|WorldtoGridCoordinates (LocalVariables|GetTheGrid) (Math|Vector|MakeVector (+ (.X (Math|Vector|BreakVector (LocalVariables|GetcharacterLocation))) (.X (Math|Vector|BreakVector (* (Class|KismetMathLibrary|GetDirectionVector (LocalVariables|GetcharacterLocation) (LocalVariables|GetEndLocation)) (* _index 100))))) (+ (.Y (Math|Vector|BreakVector (LocalVariables|GetcharacterLocation))) (.Y (Math|Vector|BreakVector (* (Class|KismetMathLibrary|GetDirectionVector (LocalVariables|GetcharacterLocation) (LocalVariables|GetEndLocation)) (* _index 100))))) 0.0)))))
            (Utilities|IsValid (Variables|/Game/BattleBotsContent/Grid/BP_GridCell.BP_GridCell_C|GetUnit _gridcell)
              (:Is%20Valid
                (for _array_element_2 (Variables|/Game/BattleBotsContent/Skills/BP_Skill.BP_Skill_C|GetSkillEffectsToApply (Utilities|Array|Get(acopy) (Variables|/Game/BattleBotsContent/Units/BP_UnitComponent.BP_UnitComponent_C|GetSlottedSkills (Variables|/Game/BattleBotsContent/Units/BP_Unit.BP_Unit_C|GetUnitComponent _asbp_unit))))
                  (Utilities|Array|Add (Variables|/Game/BattleBotsContent/Skills/BP_SkillEffect.BP_SkillEffect_C|GetTargetAlso _array_element_2) (Variables|/Game/BattleBotsContent/Grid/BP_GridCell.BP_GridCell_C|GetUnit _gridcell))))
              (:Is%20Not%20Valid
                _))
            (Default|Spawn (Variables|/Game/BattleBotsContent/Units/BP_Unit.BP_Unit_C|GetBP_UnitInteract_Component _asbp_unit) (Math|Vector|MakeVector (* (.GridLocationX (Default|WorldtoGridCoordinates (LocalVariables|GetTheGrid) (Math|Vector|MakeVector (+ (.X (Math|Vector|BreakVector (LocalVariables|GetcharacterLocation))) (.X (Math|Vector|BreakVector (* (Class|KismetMathLibrary|GetDirectionVector (LocalVariables|GetcharacterLocation) (LocalVariables|GetEndLocation)) (* _index 100))))) (+ (.Y (Math|Vector|BreakVector (LocalVariables|GetcharacterLocation))) (.Y (Math|Vector|BreakVector (* (Class|KismetMathLibrary|GetDirectionVector (LocalVariables|GetcharacterLocation) (LocalVariables|GetEndLocation)) (* _index 100))))) 0.0))) 1e+02) (* (.GridLocationY (Default|WorldtoGridCoordinates (LocalVariables|GetTheGrid) (Math|Vector|MakeVector (+ (.X (Math|Vector|BreakVector (LocalVariables|GetcharacterLocation))) (.X (Math|Vector|BreakVector (* (Class|KismetMathLibrary|GetDirectionVector (LocalVariables|GetcharacterLocation) (LocalVariables|GetEndLocation)) (* _index 100))))) (+ (.Y (Math|Vector|BreakVector (LocalVariables|GetcharacterLocation))) (.Y (Math|Vector|BreakVector (* (Class|KismetMathLibrary|GetDirectionVector (LocalVariables|GetcharacterLocation) (LocalVariables|GetEndLocation)) (* _index 100))))) 0.0))) 1e+02) 5.0) "NewEnumerator0"))
          (return true))
        (:CastFailed
          _)))
    (:CastFailed
      _))
  (return false))