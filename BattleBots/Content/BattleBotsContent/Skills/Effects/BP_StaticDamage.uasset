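; BP_StaticDamage is a skill effect that deals fixed damage to the units targeted by a skill, excluding the caster.
; Apply loops over the skill's targets and picks a hardcoded damage amount, slightly higher when the target's UnitComponent is Traced.
; It subtracts that from current health without factoring in armor, writes the stats back, and destroys any target at zero health or below.
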(fn Apply
  (params (Skill :type BP%20Skill%20Object%20Reference))
  (bind _asbp_unit (Utilities|Casting|CastToBP_Unit (Variables|/Game/BattleBotsContent/Skills/BP_Skill.BP_Skill_C|GetSourceSkillUser Skill))
    (:then
      (LocalVariables|SetunitSelf _asbp_unit)
      (bind _targetskillusers (CallFunction|GetSkillUserTargets Skill))
      (for _array_element _targetskillusers
        (bind _asbp_unit_2 (Utilities|Casting|CastToBP_Unit _array_element))
        (bind _stats (Default|GetStats _asbp_unit_2))
        (bind _asbp_unit_3 (Utilities|Casting|CastToBP_Unit _array_element))
        (if (not (== (LocalVariables|GetunitSelf) _asbp_unit_3))
          (if (Variables|/Game/BattleBotsContent/Units/BP_UnitComponent.BP_UnitComponent_C|GetTraced (Variables|/Game/BattleBotsContent/Units/BP_Unit.BP_Unit_C|GetUnitComponent _asbp_unit_3))
            (LocalVariables|Setdmg 3)
            (else
              (LocalVariables|Setdmg 2)))
          (Default|SetStats _array_element (Utilities|Struct|MakeBPS_Stats (- (.CurrentHealth (Utilities|Struct|BreakBPS_Stats _stats)) (LocalVariables|Getdmg)) (.MaxHealth (Utilities|Struct|BreakBPS_Stats _stats)) (.Armor (Utilities|Struct|BreakBPS_Stats _stats)) (.MovementRange (Utilities|Struct|BreakBPS_Stats _stats))))
          (bind _stats_2 (Default|GetStats _array_element))
          (if (<= (.CurrentHealth (Utilities|Struct|BreakBPS_Stats _stats_2)) 0)
            (Default|DestroySkillUser _array_element)))))
    (:CastFailed
      _))
  (return false))