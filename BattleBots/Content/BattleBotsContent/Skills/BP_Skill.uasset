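; BP_Skill is a BattleBots skill object that applies a list of effects to a target skill user or grid location.
; Applying runs stored updaters to modify the skill, applies each effect, then restores original attributes and effects and clears the updaters.
; GetResultSkill builds a separate updated skill by copying attributes, retargeting the existing updaters to it, and constructing fresh effects whose classes appear in a known-class list.
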(fn Initialize
  (bind _skilleffectstoapply (Variables|Default|GetSkillEffectsToApply))
  ;[1 1 1] Set the contents of the Skill to be the original content
  (Utilities|Array|Clear _skilleffectstoapply)
  (Utilities|Array|AppendArray _skilleffectstoapply (Variables|Default|GetOriginalSkillEffectsToApply))
  (bind _output_get (LocalVariables|SetTempAttributes (Variables|Default|GetOriginalSkillAttributes)))
  (Variables|Default|SetSkillAttributes _output_get)
  (Utilities|Array|Clear (Variables|Default|GetStoredSkillUpdaters))
  (return))

(fn ApplySkilltoTarget
  (params (SourceSkillUser :type BPI%20Skill%20User%20Interface) (TargetSkillUser :type BPI%20Skill%20User%20Interface))
  (Variables|Default|SetSourceSkillUser SourceSkillUser)
  (Variables|Default|SetTargetSkillUser TargetSkillUser)
  (CallFunction|ApplySkill)
  (return))

(fn ApplySkill
  (bind _self self)
  ;[1 1 1] Update skill stats first
  (for _array_element (Variables|Default|GetStoredSkillUpdaters)
    (Default|UpdateSkill _array_element _self))
  ;[1 1 1] Then, apply each SkillEffect from the Skill to the targeted SkillUser
  (for _array_element_2 (Variables|Default|GetSkillEffectsToApply)
    (Default|Apply _array_element_2 _self))
  (CallFunction|Initialize)
  (return))

(fn ApplySkilltoGridLocation
  (params (X :type Integer) (Y :type Integer) (SourceSkillUser :type BPI%20Skill%20User%20Interface))
  (Variables|Default|SetTargetGridLocationX X)
  (Variables|Default|SetTargetGridLocationY Y)
  (Variables|Default|SetSourceSkillUser SourceSkillUser)
  (CallFunction|ApplySkill)
  (return))

(fn GetResultSkill
  (bind _skilleffectstoapply (Variables|Default|GetSkillEffectsToApply))
  (bind _existingskilleffectclasses (Variables|Default|GetExistingSkillEffectClasses))
  ;[1 1 1] Create a new skill
  (bind _returnvalue (Game|ConstructObjectfromClass "BP_Skill_C" self))
  (Utilities|FlowControl|Sequence
    (:then_0
      ;[1 1 1] Copy the skill attributes
      (bind _output_get (LocalVariables|SetTempSkillAttributes (Variables|Default|GetSkillAttributes)))
      (Variables|BP_Skill_C|SetSkillAttributes _returnvalue _output_get))
    (:then_1
      ;[1 1 1] For each of my skill updaters, update the new skill's stuff rather than creating all new updaters and adding them to the new skill's personal list of skill updaters
      (for _array_element (Variables|Default|GetStoredSkillUpdaters)
        (bind _output_get_2 (Variables|/Game/BattleBotsContent/Skills/BP_SkillUpdater.BP_SkillUpdater_C|SetSkillToUpdate _array_element _returnvalue))
        (Default|UpdateSkill _array_element _output_get_2)))
    (:then_2
      ;[1 1 1] For each of my skill effects, create new skill effects to add to the new skill's list of skill effects
      (for _array_element_2 _skilleffectstoapply
        (if (>= (Utilities|Array|FindItem _existingskilleffectclasses (Utilities|GetClass _array_element_2)) 0)
          (bind _returnvalue_2 (Game|ConstructObjectfromClass (Utilities|Array|Get(acopy) _existingskilleffectclasses (Utilities|Array|FindItem _existingskilleffectclasses (Utilities|GetClass _array_element_2))) self (Variables|/Game/BattleBotsContent/Skills/BP_SkillEffect.BP_SkillEffect_C|GetGameMode (Utilities|Array|Get(acopy) _skilleffectstoapply))))
          (Utilities|Array|Add (Variables|BP_Skill_C|GetSkillEffectsToApply _returnvalue) _returnvalue_2))))
    (:then_3
      (return _returnvalue))))

(fn ClearSkillUpdaters
  (Utilities|Array|Clear (Variables|Default|GetStoredSkillUpdaters)))