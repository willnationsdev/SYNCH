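; BP_BattleGameMode is the battle game mode, holding shared state for active team, battle mode, controlled unit, controllable units and grid manager behind getters and setters.
; AcquireControllableUnits rebuilds the controllable list from BP_Unit actors whose team component matches the active team.
; On BeginPlay, SetWindowed, despite its name, applies the last supported resolution as fullscreen through r.SetRes.
; GetAttackSound is an unfinished chain of unit-name checks that returns no sound.
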(event `self.ReceiveBeginPlay`
  (`self.setWindowed`))

(event `self.ReceiveTick`
  (params (DeltaSeconds :type "Float (single-precision)")))

(fn `AcquireControllableUnits`
  (returns (ControllableUnits :type "Array of /Game/BattleBotsContent/Units/BP_Unit Object Reference"))
  (`KismetArrayLibrary.Array_Clear` (`self.ControllableUnits`))
  (bind _outactors (`GameplayStatics.GetAllActorsOfClass` "/Game/BattleBotsContent/Units/BP_Unit.BP_Unit_C"))
  (for _array_element _outactors
    (bind _team_ (`/Game/BattleBotsContent/Units/BP_UnitTeamComponent.Get Team` (`/Game/BattleBotsContent/Units/BP_Unit.BP_UnitTeamComponent` _array_element)))
    (if (`|EnumEquality` _team_ (`self.CurrentActiveTeam`))
      (`KismetArrayLibrary.Array_Add` (`self.ControllableUnits`) _array_element)))
  (return (`self.ControllableUnits`)))

(fn `GetActiveTeam`
  (returns (ActiveTeam :type "/Game/BattleBotsContent/Global/ETeamAssociation Enum"))
  (return (`self.CurrentActiveTeam`)))

(fn `getAllunits`
  (returns (allUnits :type "Array of /Game/BattleBotsContent/Units/BP_Unit Object Reference"))
  (bind _outactors (`GameplayStatics.GetAllActorsOfClass` "/Game/BattleBotsContent/Units/BP_Unit.BP_Unit_C"))
  (return _outactors))

(fn `getAttackSound`
  (returns (soundEffect :type "AmbientSound Object Reference"))
  (bind _controlledunit (`self.GetControlledUnit`))
  (bind _unitname (`/Game/BattleBotsContent/Units/BP_UnitComponent.UnitName` (`/Game/BattleBotsContent/Units/BP_Unit.UnitComponent` _controlledunit)))
  (if (== _unitname "TankBot")
    _
    (elif (== _unitname "MinonBot")
      _
      (elif (== _unitname "Minion")
        _
        (elif (== _unitname "AcidBot")
          _
          (elif (== _unitname "BerzerkBot")
            _
            (elif (== _unitname "TracerBot")
              _
              (elif (== _unitname "AcidBoss")
                _
                (elif (== _unitname "CrushBoss")
                  _
                  (elif (== _unitname "PullBoss")
                    _
                    (elif (== _unitname "HammerBot")
                      _
                      (elif (== _unitname "SniperBot")
                        _))))))))))))

(fn `GetBattleMode`
  (returns (BattleMode :type "/Game/BattleBotsContent/Global/EBattleMode Enum"))
  (return (`self.CurrentBattleMode`)))

(fn `GetControlledUnit`
  (returns (ControlledUnit :type "/Game/BattleBotsContent/Units/BP_Unit Object Reference"))
  (return (`self.ControlledUnit`)))

(fn `GetControlledUnits`
  (returns (ControllableUnits :type "Array of /Game/BattleBotsContent/Units/BP_Unit Object Reference"))
  (return (`self.ControllableUnits`)))

(fn `GetGridManager`
  (returns (GridManager :type "/Game/BattleBotsContent/Grid/BP_GridManager Object Reference"))
  (return (`self.GridManagerRef`)))

(fn `SetActiveTeam`
  (params (ActiveTeam :type "/Game/BattleBotsContent/Global/ETeamAssociation Enum" :default "NewEnumerator0"))
  (returns (ActiveTeamOut :type "/Game/BattleBotsContent/Global/ETeamAssociation Enum"))
  (bind _output_get (set `self.CurrentActiveTeam` ActiveTeam))
  (return _output_get))

(fn `SetBattleMode`
  (params (NewBattleMode :type "/Game/BattleBotsContent/Global/EBattleMode Enum" :default "NewEnumerator4"))
  (returns (BattleMode :type "/Game/BattleBotsContent/Global/EBattleMode Enum"))
  (bind _output_get (set `self.CurrentBattleMode` NewBattleMode))
  (return _output_get))

(fn `SetControlledUnit`
  (params (NewControlledUnit :type "/Game/BattleBotsContent/Units/BP_Unit Object Reference"))
  (returns (ControlledUnit :type "/Game/BattleBotsContent/Units/BP_Unit Object Reference"))
  (bind _output_get (set `self.ControlledUnit` NewControlledUnit))
  (return _output_get))

(fn `SetControlledUnits`
  (params (NewControllableUnits :type "Array of /Game/BattleBotsContent/Units/BP_Unit Object Reference (by ref)"))
  (returns (ControllableUnits :type "Array of /Game/BattleBotsContent/Units/BP_Unit Object Reference"))
  (bind _output_get (set `self.ControllableUnits` NewControllableUnits))
  (return _output_get))

(fn `SetGridManager`
  (params (NewGridManager :type "/Game/BattleBotsContent/Grid/BP_GridManager Object Reference"))
  (returns (` GridManager` :type "/Game/BattleBotsContent/Grid/BP_GridManager Object Reference"))
  (bind _output_get (set `self.GridManagerRef` NewGridManager))
  (return _output_get))

(fn `setWindowed`
  (bind _resolutions (`KismetSystemLibrary.GetSupportedFullscreenResolutions`))
  (bind (_x _y) (break `IntPoint` (`KismetArrayLibrary.Array_Get` _resolutions (`KismetArrayLibrary.Array_LastIndex` _resolutions))))
  (`KismetSystemLibrary.ExecuteConsoleCommand` (`KismetStringLibrary.Concat_StrStr` "r.SetRes " (`KismetStringLibrary.Conv_IntToString` _x) "x" (`KismetStringLibrary.Conv_IntToString` _y) "f")))

(fn `UserConstructionScript`)