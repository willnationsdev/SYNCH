(event `self.ReceiveBeginPlay`)

(event `self.ReceiveActorBeginOverlap`
  (params (OtherActor :type "Actor Object Reference")))

(event `self.ReceiveTick`
  (params (DeltaSeconds :type "Float (single-precision)")))

(event `self.Create`
  (bind _returnvalue (`GameplayStatics.GetGameMode`))
  (bind _turnstolive (`self.TurnsToLive`))
  (bind _currentunit (`self.CurrentUnit`))
  (bind _thegrid (`self.TheGrid`))
  (bind _currentunit_2 (`self.CurrentUnit`))
  (bind _unitcomponent (`/Game/BattleBotsContent/Units/BP_Unit.UnitComponent` _currentunit))
  (bind _unitcomponent_2 (`/Game/BattleBotsContent/Units/BP_Unit.UnitComponent` _currentunit_2))
  (bind (_gridlocationx _gridlocationy) (`/Game/BattleBotsContent/Grid/BP_GridManager.WorldToGridCoordinates` _thegrid (`self.K2_GetActorLocation` self)))
  (bind (_currenthealth _maxhealth _armor _movementrange) (break `/Game/BattleBotsContent/Units/BPS_Stats` (`/Game/BattleBotsContent/Units/BP_UnitComponent.Stats` _unitcomponent_2)))
  (bind (_currenthealth_2 _maxhealth_2 _armor_2 _movementrange_2) (break `/Game/BattleBotsContent/Units/BPS_Stats` (`/Game/BattleBotsContent/Units/BP_UnitComponent.Stats` _unitcomponent)))
  (set `self.TurnsToLive` 2)
  (if (== _turnstolive 0) :!label _label
    (`/Engine/EditorBlueprintResources/StandardMacros.IsValid` _currentunit_2
      (:`Is Valid`
        (bind _asbpi_battle_manager (cast `/Game/BattleBotsContent/Global/BPI_BattleManager` (`GameplayStatics.GetGameMode`)))
        (bind _activeteam (`/Game/BattleBotsContent/Global/BPI_BattleManager.GetActiveTeam` _asbpi_battle_manager))
        (set `self.ActiveTeam` _activeteam)
        (if (`|EnumEquality` (`self.ActiveTeam`) (`/Game/BattleBotsContent/Units/BP_UnitTeamComponent.Team` (`/Game/BattleBotsContent/Units/BP_Unit.BP_UnitTeamComponent` _currentunit_2)))
          (set `/Game/BattleBotsContent/Units/BP_UnitComponent.Stats` (make `/Game/BattleBotsContent/Units/BPS_Stats` _currenthealth _maxhealth _armor (+ _movementrange (`self.originalStat`))) _unitcomponent_2)
          (`self.K2_DestroyActor` :!label _label_2)))
      (:`Is Not Valid`
        (goto _label_2)))
    (else
      (`/Engine/EditorBlueprintResources/StandardMacros.DecrementInt` _turnstolive
        (:`  `
          (`|ExecutionSequence`
            (:`then_0`
              (bind _asbpi_battle_manager_2 (cast `/Game/BattleBotsContent/Global/BPI_BattleManager` _returnvalue))
              (bind _activeteam_2 (`/Game/BattleBotsContent/Global/BPI_BattleManager.GetActiveTeam` _asbpi_battle_manager_2))
              (set `self.ActiveTeam` _activeteam_2))
            (:`then_1`
              (bind _asbpi_grid_managing_game_mode (cast `/Game/BattleBotsContent/Grid/BPI_GridManagingGameMode` _returnvalue))
              (bind _gridmanager (`/Game/BattleBotsContent/Grid/BPI_GridManagingGameMode.GetGridManager` _asbpi_grid_managing_game_mode))
              (set `self.TheGrid` _gridmanager))
            (:`then_2`
              (bind _isempty (`/Game/BattleBotsContent/Grid/BP_GridManager.GridCellIsEmpty` _thegrid _gridlocationx _gridlocationy))
              (if _isempty
                (set `self.CurrentUnit` null)
                (else
                  (`/Engine/EditorBlueprintResources/StandardMacros.IsValid` (`self.CurrentUnit`)
                    (:`Is Valid`
                      (bind _asbpi_battle_manager_3 (cast `/Game/BattleBotsContent/Global/BPI_BattleManager` (`GameplayStatics.GetGameMode`) :!label _label_3))
                      (bind _activeteam_3 (`/Game/BattleBotsContent/Global/BPI_BattleManager.GetActiveTeam` _asbpi_battle_manager_3))
                      (set `self.ActiveTeam` _activeteam_3)
                      (if (`|EnumEquality` (`self.ActiveTeam`) (`/Game/BattleBotsContent/Units/BP_UnitTeamComponent.Team` (`/Game/BattleBotsContent/Units/BP_Unit.BP_UnitTeamComponent` _currentunit)))
                        (set `/Game/BattleBotsContent/Units/BP_UnitComponent.Stats` (make `/Game/BattleBotsContent/Units/BPS_Stats` _currenthealth_2 _maxhealth_2 _armor_2 (- _movementrange_2 (`self.originalStat`))) _unitcomponent)))
                    (:`Is Not Valid`
                      (bind _outactors (`GameplayStatics.GetAllActorsOfClass` "/Game/BattleBotsContent/Units/BP_Unit.BP_Unit_C"))
                      (for _array_element _outactors
                        (if (== (`self.K2_GetActorLocation` _array_element) (`self.K2_GetActorLocation` self) :`ErrorTolerance` 50.0)
                          (set `self.CurrentUnit` _array_element)
                          (goto _label_3))))))))))))))

(event `self.Reset`
  (goto _label))

(fn `UserConstructionScript`
  (`parent.UserConstructionScript`))