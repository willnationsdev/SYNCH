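; BP_Interact_Trc is an interact actor that applies a temporary Traced status to a grid unit.
; On Create, it gets the grid manager through the game mode, finds the unit in the cell at its location, flags that unit's UnitComponent as Traced and starts a countdown.
; Each Reset call decrements the countdown and reapplies the flag, until zero clears it and destroys the actor.
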(event `self.ReceiveBeginPlay`)

(event `self.ReceiveActorBeginOverlap`
  (params (OtherActor :type "Actor Object Reference")))

(event `self.ReceiveTick`
  (params (DeltaSeconds :type "Float (single-precision)")))

(event `self.Create`
  (bind _asbpi_grid_managing_game_mode (cast `/Game/BattleBotsContent/Grid/BPI_GridManagingGameMode` (`GameplayStatics.GetGameMode`)))
  (bind _gridmanager (`/Game/BattleBotsContent/Grid/BPI_GridManagingGameMode.GetGridManager` _asbpi_grid_managing_game_mode))
  (bind (_gridlocationx _gridlocationy) (`/Game/BattleBotsContent/Grid/BP_GridManager.WorldToGridCoordinates` _gridmanager (`self.K2_GetActorLocation` self)))
  (bind _gridcell (`/Game/BattleBotsContent/Grid/BP_GridManager.GetGridCellFromCoordinates` _gridmanager _gridlocationx _gridlocationy))
  (set `self.UnitRef` (`/Game/BattleBotsContent/Grid/BP_GridCell.Unit` _gridcell))
  (set `/Game/BattleBotsContent/Units/BP_UnitComponent.Traced` true (`/Game/BattleBotsContent/Units/BP_Unit.UnitComponent` (`self.UnitRef`)))
  (set `self.Countdown` (`self.MaxCountdown`)))

(event `self.Reset`
  (bind _result (`/Engine/EditorBlueprintResources/StandardMacros.DecrementInt` (`self.Countdown`))
    (:`  `
      (if (== _result 0)
        (set `/Game/BattleBotsContent/Units/BP_UnitComponent.Traced` false (`/Game/BattleBotsContent/Units/BP_Unit.UnitComponent` (`self.UnitRef`)))
        (`self.K2_DestroyActor`)
        (else
          (set `/Game/BattleBotsContent/Units/BP_UnitComponent.Traced` true (`/Game/BattleBotsContent/Units/BP_Unit.UnitComponent` (`self.UnitRef`))))))))

(fn `UserConstructionScript`
  (`parent.UserConstructionScript`))