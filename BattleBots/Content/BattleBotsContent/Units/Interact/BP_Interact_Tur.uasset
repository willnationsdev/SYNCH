(event `self.ReceiveBeginPlay`)

(event `self.ReceiveActorBeginOverlap`
  (params (OtherActor :type "Actor Object Reference")))

(event `self.ReceiveTick`
  (params (DeltaSeconds :type "Float (single-precision)")))

(event `self.Create`
  (bind _linker (`self.Linker`))
  (bind _linker_2 (`self.Linker`))
  (`/Engine/EditorBlueprintResources/StandardMacros.IsValid` (`self.Linker`)
    (:`Is Not Valid`
      (bind _returnvalue (`|SpawnActorFromClass` "/Game/BattleBotsContent/Units/BP_Unit.BP_Unit_C" (`KismetMathLibrary.MakeTransform` (.location (`self.GetTransform` self)) (struct :`Yaw` 90.0 :`Roll` -90.0) (1.0 1.0 1.0)) "Undefined" "OverrideRootScale" null self))
      (set `self.Linker` _returnvalue)
      (`/Game/BattleBotsContent/Units/BP_UnitComponent.Initialize` (`/Game/BattleBotsContent/Units/BP_Unit.UnitComponent` _linker) "Turret")
      (`PaperFlipbookComponent.SetFlipbook` (`/Game/BattleBotsContent/Units/BP_Unit.Flipbook` _linker) "/Game/BattleBotsContent/UI/BattleUI/Materials/TF_Interact/TF_Turret2.TF_Turret2")
      (`PaperFlipbookComponent.SetFlipbook` (`/Game/BattleBotsContent/Units/BP_Unit.HUDTeam` _linker) null)
      (bind _asbpi_grid_managing_game_mode (cast `/Game/BattleBotsContent/Grid/BPI_GridManagingGameMode` (`GameplayStatics.GetGameMode`)))
      (bind _gridmanager (`/Game/BattleBotsContent/Grid/BPI_GridManagingGameMode.GetGridManager` _asbpi_grid_managing_game_mode))
      (bind (_gridlocationx _gridlocationy) (`/Game/BattleBotsContent/Grid/BP_GridManager.WorldToGridCoordinates` _gridmanager (`self.K2_GetActorLocation` _linker_2)))
      (`/Game/BattleBotsContent/Grid/BP_GridManager.PlaceUnit` _gridmanager _gridlocationx _gridlocationy _linker_2))))

(event `self.Reset`
  (bind _bp_unitteamcomponent (`/Game/BattleBotsContent/Units/BP_Unit.BP_UnitTeamComponent` (`self.Linker`)))
  (bind _asbpi_battle_manager (cast `/Game/BattleBotsContent/Global/BPI_BattleManager` (`GameplayStatics.GetGameMode`)))
  (bind _activeteam (`/Game/BattleBotsContent/Global/BPI_BattleManager.GetActiveTeam` _asbpi_battle_manager))
  (`/Game/BattleBotsContent/Units/BP_UnitTeamComponent.Set Team` (`/Game/BattleBotsContent/Units/BP_Unit.BP_UnitTeamComponent` (`self.Linker`)) _activeteam)
  (`/Game/BattleBotsContent/Units/BP_UnitTeamComponent.MarkLinkOrSkillActionAsActivated` _bp_unitteamcomponent)
  (`/Game/BattleBotsContent/Units/BP_UnitTeamComponent.ResetActions` _bp_unitteamcomponent)
  (`/Game/BattleBotsContent/Units/BP_UnitTeamComponent.MoveActivation` _bp_unitteamcomponent))

(fn `UserConstructionScript`
  (`parent.UserConstructionScript`))