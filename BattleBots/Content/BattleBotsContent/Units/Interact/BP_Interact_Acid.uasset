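; BP_Interact_Acid is an acid hazard on the battle grid that damages the unit standing on its cell.
; Activate checks the cell through the grid manager, clearing CurrentUnit when empty, otherwise reusing it or finding a BP_Unit by location.
; DealDamage hurts that unit only while its team is active, hitting harder if Traced, ignoring Armor, and destroys it when health runs out.
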(event `self.ReceiveBeginPlay`)

(event `self.ReceiveActorBeginOverlap`
  (params (OtherActor :type "Actor Object Reference")))

(event `self.ReceiveTick`
  (params (DeltaSeconds :type "Float (single-precision)")))

(fn `Activate`
  (bind _returnvalue (`GameplayStatics.GetGameMode`))
  (bind _thegrid (`self.TheGrid`))
  (bind (_gridlocationx _gridlocationy) (`/Game/BattleBotsContent/Grid/BP_GridManager.WorldToGridCoordinates` _thegrid (`self.K2_GetActorLocation` self)))
  (`|ExecutionSequence`
    (:`then_0`
      (bind _asbpi_battle_manager (cast `/Game/BattleBotsContent/Global/BPI_BattleManager` _returnvalue))
      (bind _activeteam (`/Game/BattleBotsContent/Global/BPI_BattleManager.GetActiveTeam` _asbpi_battle_manager))
      (set `self.active team` _activeteam))
    (:`then_1`
      (bind _asbpi_grid_managing_game_mode (cast `/Game/BattleBotsContent/Grid/BPI_GridManagingGameMode` _returnvalue))
      (bind _gridmanager (`/Game/BattleBotsContent/Grid/BPI_GridManagingGameMode.GetGridManager` _asbpi_grid_managing_game_mode))
      (set `self.TheGrid` _gridmanager))
    (:`then_2`
      (bind _isempty (`/Game/BattleBotsContent/Grid/BP_GridManager.GridCellIsEmpty` _thegrid _gridlocationx _gridlocationy))
      (if _isempty
        (set `self.CurrentUnit` null)
        (else
          (`/Engine/EditorBlueprintResources/StandardMacros.IsValid` (`self.CurrentUnit`)
            (:`Is Valid`
              (`self.dealDamage` :!label _label))
            (:`Is Not Valid`
              (bind _outactors (`GameplayStatics.GetAllActorsOfClass` "/Game/BattleBotsContent/Units/BP_Unit.BP_Unit_C"))
              (for _array_element _outactors
                (if (== (`self.K2_GetActorLocation` _array_element) (`self.K2_GetActorLocation` self) :`ErrorTolerance` 50.0)
                  (set `self.CurrentUnit` _array_element)
                  (goto _label))))))))))

(fn `dealDamage`
  (bind _currentunit (`self.CurrentUnit`))
  (bind _unitcomponent (`/Game/BattleBotsContent/Units/BP_Unit.UnitComponent` _currentunit))
  (bind (_currenthealth _maxhealth _armor _movementrange) (break `/Game/BattleBotsContent/Units/BPS_Stats` (`/Game/BattleBotsContent/Units/BP_UnitComponent.Stats` _unitcomponent)))
  (bind _asbpi_battle_manager (cast `/Game/BattleBotsContent/Global/BPI_BattleManager` (`GameplayStatics.GetGameMode`)))
  (bind _activeteam (`/Game/BattleBotsContent/Global/BPI_BattleManager.GetActiveTeam` _asbpi_battle_manager))
  (set `self.active team` _activeteam)
  (if (`|EnumEquality` (`self.active team`) (`/Game/BattleBotsContent/Units/BP_UnitTeamComponent.Team` (`/Game/BattleBotsContent/Units/BP_Unit.BP_UnitTeamComponent` _currentunit)))
    (if (`/Game/BattleBotsContent/Units/BP_UnitComponent.Traced` _unitcomponent)
      (set `self.Dmg` 3)
      (else
        (set `self.Dmg` 2)))
    (set `/Game/BattleBotsContent/Units/BP_UnitComponent.Stats` (make `/Game/BattleBotsContent/Units/BPS_Stats` (- _currenthealth (`self.Dmg`)) _maxhealth _armor _movementrange) _unitcomponent)
    (if (< _currenthealth 1)
      (`self.K2_DestroyActor` (`self.CurrentUnit`)))))

(fn `UserConstructionScript`)