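; BP_Interact_Min is an interactable that spawns a linked Minion unit for the active team on a grid battlefield.
; Once AllowCreate sets its flag, Create spawns a BP_Unit if none is linked, then sets up its flipbooks and team color.
; It places the unit on the grid, resets its actions and registers it with the battle HUD.
; Reset destroys both unit and interactable when the unit's team is active.
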(event `self.ReceiveBeginPlay`)

(event `self.ReceiveActorBeginOverlap`
  (params (OtherActor :type "Actor Object Reference")))

(event `self.ReceiveTick`
  (params (DeltaSeconds :type "Float (single-precision)")))

(event `self.Create`
  (bind _returnvalue (`GameplayStatics.GetGameMode`))
  (bind _linker (`self.Linker`))
  (bind _linker_2 (`self.Linker`))
  (bind _bp_unitteamcomponent (`/Game/BattleBotsContent/Units/BP_Unit.BP_UnitTeamComponent` (`self.Linker`)))
  (bind _flipbook (`/Game/BattleBotsContent/Units/BP_Unit.Flipbook` _linker))
  (bind _hudteam (`/Game/BattleBotsContent/Units/BP_Unit.HUDTeam` _linker))
  (if (`self.allow`)
    (`/Engine/EditorBlueprintResources/StandardMacros.IsValid` (`self.Linker`)
      (:`Is Not Valid`
        (bind _returnvalue_2 (`|SpawnActorFromClass` "/Game/BattleBotsContent/Units/BP_Unit.BP_Unit_C" (`KismetMathLibrary.MakeTransform` (.location (`self.GetTransform` self)) (struct :`Yaw` 90.0 :`Roll` -90.0) (1.0 1.0 1.0)) "AlwaysSpawn" "OverrideRootScale" null self))
        (set `self.Linker` _returnvalue_2)
        (`/Game/BattleBotsContent/Units/BP_UnitComponent.Initialize` (`/Game/BattleBotsContent/Units/BP_Unit.UnitComponent` _linker) "Minion")
        (`PaperFlipbookComponent.SetFlipbook` _flipbook "/Game/BattleBotsContent/UI/BattleUI/Materials/AL_Units/AL_Min2.AL_Min2")
        (`SceneComponent.SetWorldScale3D` _flipbook (0.95 0.95 0.95))
        (`SceneComponent.K2_AddLocalRotation` _flipbook (struct :`Yaw` 180.0) false false)
        (`PaperFlipbookComponent.SetFlipbook` _hudteam "/Game/BattleBotsContent/UI/BattleUI/Materials/TF_Teams_Flipbook.TF_Teams_Flipbook")
        (bind _asbpi_battle_manager (cast `/Game/BattleBotsContent/Global/BPI_BattleManager` _returnvalue))
        (bind _activeteam (`/Game/BattleBotsContent/Global/BPI_BattleManager.GetActiveTeam` _asbpi_battle_manager))
        (`/Game/BattleBotsContent/Units/BP_UnitTeamComponent.Set Team` (`/Game/BattleBotsContent/Units/BP_Unit.BP_UnitTeamComponent` _linker) _activeteam)
        (switch `/Game/BattleBotsContent/Global/ETeamAssociation` _activeteam
          (:`NewEnumerator1`
            (`PaperFlipbookComponent.SetSpriteColor` _hudteam (struct :`R` 0.233058 :`G` 0.357173 :`B` 1.0 :`A` 1.0)))
          (:`NewEnumerator2`
            (`PaperFlipbookComponent.SetSpriteColor` _hudteam (struct :`R` 1.0 :`G` 0.089066 :`B` 0.35083 :`A` 1.0))))
        (bind _asbpi_grid_managing_game_mode (cast `/Game/BattleBotsContent/Grid/BPI_GridManagingGameMode` _returnvalue))
        (bind _gridmanager (`/Game/BattleBotsContent/Grid/BPI_GridManagingGameMode.GetGridManager` _asbpi_grid_managing_game_mode))
        (bind (_gridlocationx _gridlocationy) (`/Game/BattleBotsContent/Grid/BP_GridManager.WorldToGridCoordinates` _gridmanager (`self.K2_GetActorLocation` _linker_2)))
        (`/Game/BattleBotsContent/Grid/BP_GridManager.PlaceUnit` _gridmanager _gridlocationx _gridlocationy _linker_2)
        (`/Game/BattleBotsContent/Units/BP_UnitTeamComponent.MarkLinkOrSkillActionAsActivated` _bp_unitteamcomponent)
        (`/Game/BattleBotsContent/Units/BP_UnitTeamComponent.ResetActions` _bp_unitteamcomponent)
        (bind _outactors (`GameplayStatics.GetAllActorsOfClass` "/Game/BattleBotsContent/UI/BattleUI/BP_BattleHUD.BP_BattleHUD_C"))
        (`KismetArrayLibrary.Array_AddUnique` (`/Game/BattleBotsContent/UI/BattleUI/BP_BattleHUD.CurrentBP_Units` (`KismetArrayLibrary.Array_Get` _outactors)) (`self.Linker`))))))

(event `self.Reset`
  (bind _linker (`self.Linker`))
  (bind _asbpi_battle_manager (cast `/Game/BattleBotsContent/Global/BPI_BattleManager` (`GameplayStatics.GetGameMode`)))
  (bind _activeteam (`/Game/BattleBotsContent/Global/BPI_BattleManager.GetActiveTeam` _asbpi_battle_manager))
  (if (`|EnumEquality` _activeteam (`/Game/BattleBotsContent/Units/BP_UnitTeamComponent.Team` (`/Game/BattleBotsContent/Units/BP_Unit.BP_UnitTeamComponent` _linker)))
    (`self.K2_DestroyActor` _linker)
    (`self.K2_DestroyActor`)))

(fn `allowCreate`
  (set `self.allow` true))

(fn `UserConstructionScript`
  (`parent.UserConstructionScript`))