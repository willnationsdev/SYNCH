(event `self.ReceiveBeginPlay`)

(event `self.ReceiveActorBeginOverlap`
  (params (OtherActor :type "Actor Object Reference")))

(event `self.ReceiveTick`
  (params (DeltaSeconds :type "Float (single-precision)")))

(event `self.Create`
  (set `self.TurnsToLive` 3)
  (bind _asbpw_unit_wdget_comp (cast `/Game/BattleBotsContent/UI/UnitWidget/BPW_UnitWdgetComp` (`WidgetComponent.GetUserWidgetObject` (`self.Widget`))))
  (`/Game/BattleBotsContent/UI/UnitWidget/BPW_UnitWdgetComp.SetHealth` _asbpw_unit_wdget_comp 3 3)
  (`/Game/BattleBotsContent/UI/UnitWidget/BPW_UnitWdgetComp.changetextcolor` _asbpw_unit_wdget_comp))

(event `self.Reset`
  (bind _returnvalue (`GameplayStatics.GetGameMode`))
  (bind _turnstolive (`self.TurnsToLive`))
  (bind _currentunit (`self.CurrentUnit`))
  (bind _thegrid (`self.TheGrid`))
  (bind _thegrid_2 (`self.TheGrid`))
  (bind _unitcomponent (`/Game/BattleBotsContent/Units/BP_Unit.UnitComponent` _currentunit))
  (bind (_gridlocationx _gridlocationy) (`/Game/BattleBotsContent/Grid/BP_GridManager.WorldToGridCoordinates` _thegrid (`self.K2_GetActorLocation` self)))
  (bind (_gridlocationx_2 _gridlocationy_2) (`/Game/BattleBotsContent/Grid/BP_GridManager.WorldToGridCoordinates` _thegrid_2 (`self.K2_GetActorLocation` self)))
  (bind (_currenthealth _maxhealth _armor _movementrange) (break `/Game/BattleBotsContent/Units/BPS_Stats` (`/Game/BattleBotsContent/Units/BP_UnitComponent.Stats` _unitcomponent)))
  (bind _result (`/Engine/EditorBlueprintResources/StandardMacros.DecrementInt` _turnstolive)
    (:`  `
      (if (== _turnstolive 0)
        (`|ExecutionSequence`
          (:`then_0`
            (bind _asbpw_unit_wdget_comp (cast `/Game/BattleBotsContent/UI/UnitWidget/BPW_UnitWdgetComp` (`WidgetComponent.GetUserWidgetObject` (`self.Widget`)) :!label _label))
            (`/Game/BattleBotsContent/UI/UnitWidget/BPW_UnitWdgetComp.SetHealth` _asbpw_unit_wdget_comp _result 3)
            (`|ExecutionSequence`
              (:`then_0`
                (bind _asbpi_battle_manager (cast `/Game/BattleBotsContent/Global/BPI_BattleManager` _returnvalue))
                (bind _activeteam (`/Game/BattleBotsContent/Global/BPI_BattleManager.GetActiveTeam` _asbpi_battle_manager))
                (set `self.ActiveTeam` _activeteam))
              (:`then_1`
                (bind _asbpi_grid_managing_game_mode (cast `/Game/BattleBotsContent/Grid/BPI_GridManagingGameMode` _returnvalue))
                (bind _gridmanager (`/Game/BattleBotsContent/Grid/BPI_GridManagingGameMode.GetGridManager` _asbpi_grid_managing_game_mode))
                (set `self.TheGrid` _gridmanager))
              (:`then_2`
                (bind _isempty (`/Game/BattleBotsContent/Grid/BP_GridManager.GridCellIsEmpty` _thegrid_2 _gridlocationx_2 _gridlocationy_2))
                (if _isempty
                  (set `self.CurrentUnit` null)
                  (else
                    (`/Engine/EditorBlueprintResources/StandardMacros.IsValid` (`self.CurrentUnit`)
                      (:`Is Valid`
                        _)
                      (:`Is Not Valid`
                        (bind _gridcell (`/Game/BattleBotsContent/Grid/BP_GridManager.GetGridCellFromCoordinates` _thegrid _gridlocationx _gridlocationy))
                        (bind _unit (`/Game/BattleBotsContent/Grid/BP_GridCell.Unit` _gridcell))
                        (`/Engine/EditorBlueprintResources/StandardMacros.IsValid` _unit
                          (:`Is Valid`
                            (set `self.CurrentUnit` _unit)))))
                    (if (`|EnumEquality` (`self.ActiveTeam`) (`/Game/BattleBotsContent/Units/BP_UnitTeamComponent.Team` (`/Game/BattleBotsContent/Units/BP_Unit.BP_UnitTeamComponent` _currentunit)))
                      (if (`/Game/BattleBotsContent/Units/BP_UnitComponent.Traced` _unitcomponent)
                        (set `self.Dmg` 3)
                        (else
                          (set `self.Dmg` 2)))
                      (set `/Game/BattleBotsContent/Units/BP_UnitComponent.Stats` (make `/Game/BattleBotsContent/Units/BPS_Stats` (- _currenthealth (`self.Dmg`)) _maxhealth _armor _movementrange) _unitcomponent)
                      (if (<= _currenthealth 0)
                        (`self.K2_DestroyActor` (`self.CurrentUnit`)))))))))
          (:`then_1`
            (`self.K2_DestroyActor`)))
        (else
          (goto _label))))))

(fn `UserConstructionScript`
  (`parent.UserConstructionScript`))