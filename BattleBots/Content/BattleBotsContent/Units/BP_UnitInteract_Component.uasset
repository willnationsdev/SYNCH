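; Unit component that spawns grid interactables (acid pit, minion, tar pit or trace) at a given location.
; Spawn gets the grid manager from the game mode, maps the type to an actor class, then spawns it and calls its Create, with type-specific setup.
; Only acid pits check the location first: one already there gets Create again, and a cell with another interactable is left alone.
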(event EventBeginPlay)

(event EventTick
  (params (DeltaSeconds :type Float%20%28single-precision%29)))

(fn Spawn
  (params (Transform :type Vector) (Type :type EInteractables%20Enum))
  (bind _asbpi_grid_managing_game_mode (Utilities|Casting|CastToBPI_GridManagingGameMode (Game|GetGameMode))
    (:then
      (bind _gridmanager (Default|GetGridManager _asbpi_grid_managing_game_mode))
      (LocalVariables|SetTheGrid _gridmanager)
      (switch Utilities|FlowControl|Switch|SwitchonEInteractables Type
        (:NewEnumerator0
          (bind _output_get (Variables|Default|SetType "/Game/BattleBotsContent/Units/Interact/BP_Interact_Aci.BP_Interact_Aci_C"))
          (Variables|Default|SetSearchType _output_get)
          (bind _outactors (Actor|GetAllActorsOfClass (Variables|Default|GetSearchType)))
          (for _array_element _outactors
            (if (Math|Vector|Equal(Vector) (Transformation|GetActorLocation _array_element) Transform 0.0001)
              (bind _asbp_interact_aci (Utilities|Casting|CastToBP_Interact_Aci _array_element)
                (:then
                  (Default|Create _asbp_interact_aci))
                (:CastFailed
                  _))
              (return true)))
          (bind _gridcell (Default|GetGridCellfromCoordinates (LocalVariables|GetTheGrid) (.GridLocationX (Default|WorldtoGridCoordinates (LocalVariables|GetTheGrid) Transform)) (.GridLocationY (Default|WorldtoGridCoordinates (LocalVariables|GetTheGrid) Transform))))
          (Utilities|IsValid (Variables|/Game/BattleBotsContent/Grid/BP_GridCell.BP_GridCell_C|GetInteractable _gridcell)
            (:Is%20Valid
              _)
            (:Is%20Not%20Valid
              (bind _returnvalue (Game|SpawnActorfromClass (Variables|Default|GetType) (Math|Conversions|ToTransform(Vector) Transform) "AlwaysSpawn" 0 0 :!label _label))
              (bind _asbp_interact_min (Utilities|Casting|CastToBP_Interact_Min _returnvalue)
                (:then
                  (Default|AllowCreate _asbp_interact_min)
                  (Default|Create _asbp_interact_min))
                (:CastFailed
                  (bind _asbp_interact_aci_2 (Utilities|Casting|CastToBP_Interact_Aci _returnvalue)
                    (:then
                      (Transformation|SetActorRotation _asbp_interact_aci_2 "0,90.000000,-90.000000")
                      (Default|Create _asbp_interact_aci_2))
                    (:CastFailed
                      (bind _asbp_interact_tar (Utilities|Casting|CastToBP_Interact_Tar _returnvalue)
                        (:then
                          (Transformation|SetActorRotation _asbp_interact_tar "0,0.000000,90.000000")
                          (Default|Create _asbp_interact_tar))
                        (:CastFailed
                          (bind _asbp_interact_trc (Utilities|Casting|CastToBP_Interact_Trc _returnvalue)
                            (:then
                              (Default|Create _asbp_interact_trc))
                            (:CastFailed
                              _)))))))))))
        (:NewEnumerator2
          (Variables|Default|SetType "/Game/BattleBotsContent/Units/Interact/BP_Interact_Min.BP_Interact_Min_C")
          (goto _label))
        (:NewEnumerator4
          (Variables|Default|SetType "/Game/BattleBotsContent/Units/Interact/BP_Interact_Tar.BP_Interact_Tar_C")
          (goto _label))
        (:NewEnumerator5
          (Variables|Default|SetType "/Game/BattleBotsContent/Units/Interact/BP_Interact_Trc.BP_Interact_Trc_C")
          (goto _label)))
      (return true))
    (:CastFailed
      (return false))))