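; Unit component that sets up a BattleBots unit's stats, idle flipbook and slotted skills from data tables when Initialize receives a unit name.
; Each skill name becomes a skill object, with its effects constructed from DT_SkillDefinitions.
; Names missing there fall back to DT_SkillLinkDefinitions, producing a BP_Link effect whose SkillUpdater holds stat-delta and effect-modifier mods.
; Effect modifiers are created only for classes listed in ExistingSkillEffectModifierClasses.
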(event EventBeginPlay
  (if (Variables|Default|GetisRuntimeSpawned)
    _))

(event EventTick
  (params (DeltaSeconds :type Float%20%28single-precision%29)))

(fn Initialize
  (params (NewUnitName :type Name))
  ;[1 1 1] Assign and validate the unit name
  (bind _output_get (Variables|Default|SetUnitName NewUnitName))
  (bind _returnvalue (Utilities|GetDataTableRow "/Game/BattleBotsContent/Units/DT_UnitDefinitions.DT_UnitDefinitions" _output_get)
    (:then
      ;[1 1 1] Initialize the unit's stats from the data table
      (Variables|Default|SetStats (.UnitStats (Utilities|Struct|BreakBPS_UnitDefinition _returnvalue)))
      ;[1 1 1] Set animation
      (Sprite|SetFlipbook (Utilities|Array|Get(acopy) (Actor|GetComponentsByClass (Components|GetOwner) "/Script/Paper2D.PaperFlipbookComponent")) (.IdleAnimation (Utilities|Struct|BreakBPS_UnitDefinition _returnvalue)))
      ;[1 1 1] Clear out the skills. Then, for each Skill mapped to the unit in the data table...
      (Utilities|Array|Clear (Variables|Default|GetSlottedSkills))
      (for _array_element (.SkillNames (Utilities|Struct|BreakBPS_UnitDefinition _returnvalue))
        ;[1 1 1] Create the skill object
        (bind _returnvalue_2 (Game|ConstructObjectfromClass (Variables|Default|GetSkillObjectClass) self))
        ;[1 1 1] Validate whether the Skill has a definition
        (bind _returnvalue_3 (Utilities|GetDataTableRow "/Game/BattleBotsContent/Skills/DT_SkillDefinitions.DT_SkillDefinitions" _array_element)
          (:then
            ;[1 1 1] Create each effect involved in the skill and add it to its list of original effects
            (for _array_element_2 (.Effects (Utilities|Struct|BreakBPS_SkillDefinition _returnvalue_3))
              (bind _returnvalue_4 (Game|ConstructObjectfromClass _array_element_2 _returnvalue_2 (Game|GetGameMode)))
              (Utilities|Array|Add (Variables|/Game/BattleBotsContent/Skills/BP_Skill.BP_Skill_C|GetOriginalSkillEffectsToApply _returnvalue_2) _returnvalue_4))
            ;[1 1 1] Initialize the skill's attributes
            (Variables|/Game/BattleBotsContent/Skills/BP_Skill.BP_Skill_C|SetOriginalSkillAttributes _returnvalue_2 (.Attributes (Utilities|Struct|BreakBPS_SkillDefinition _returnvalue_3)))
            (Default|Initialize _returnvalue_2)
            (Variables|/Game/BattleBotsContent/Skills/BP_Skill.BP_Skill_C|SetSkillDescription _returnvalue_2 (.SkillDescription (Utilities|Struct|BreakBPS_SkillDefinition _returnvalue_3)))
            ;[1 1 1] Add it to the Unit's skills, Move on to Links
            (Utilities|Array|Add (Variables|Default|GetSlottedSkills) _returnvalue_2))
          (:RowNotFound
            ;[1 1 1] Validate whether the skill has a link definition
            (bind _returnvalue_5 (Utilities|GetDataTableRow "/Game/BattleBotsContent/Skills/DT_SkillLinkDefinitions.DT_SkillLinkDefinitions" _array_element)
              (:then
                ;[1 1 1] Initialize the description of the skill
                (Variables|/Game/BattleBotsContent/Skills/BP_Skill.BP_Skill_C|SetSkillDescription _returnvalue_2 (.LinkSkillDescription (Utilities|Struct|BreakBPS_SkillModDefinition _returnvalue_5)))
                (Variables|/Game/BattleBotsContent/Skills/BP_Skill.BP_Skill_C|SetOriginalSkillAttributes _returnvalue_2 (.LinkSkillNativeAttributes (Utilities|Struct|BreakBPS_SkillModDefinition _returnvalue_5)))
                ;[1 1 1] Create a SkillUpdater to add to the Link skill, filling it with crafted SkillMods drawn from DT_SkillLinkDefinitions
                ;;[1 0.005335 0] This section must be updated to include any newly defined SkillMod types!
                ;;;[1 1 1] Make the Updater. For each intended Mod, add it to the Updater's list of mods
                (bind _returnvalue_6 (Game|ConstructObjectfromClass "/Game/BattleBotsContent/Skills/BP_SkillUpdater.BP_SkillUpdater_C" _returnvalue_2 _returnvalue_2))
                (for (_array_element_3 _array_index) (.Mods (Utilities|Struct|BreakBPS_SkillModDefinition _returnvalue_5))
                  (bind _asbp_mod_stat_delta (Utilities|Casting|CastToBP_ModStatDeltaClass _array_element_3)
                    (:then
                      ;;[1 1 1] Create the SkillMod to be added to the Updater
                      (bind _returnvalue_7 (Game|ConstructObjectfromClass _asbp_mod_stat_delta _returnvalue_6 (Utilities|Array|Get(acopy) (.Attributes (Utilities|Struct|BreakBPS_SkillModDefinition _returnvalue_5)) _array_index)))
                      (Utilities|Array|Add (Variables|/Game/BattleBotsContent/Skills/BP_SkillUpdater.BP_SkillUpdater_C|GetSkillMods _returnvalue_6) _returnvalue_7))
                    (:CastFailed
                      (Utilities|Casting|CastToBP_SkillEffectModifierClass _array_element_3)
                      (CallFunction|HandleSkillModsforEffects _array_element_3 _returnvalue_6))))
                ;;[1 1 1] Create the actual SkillEffect, set its Updater, and add it to the Skill's Effects
                (bind _returnvalue_8 (Game|ConstructObjectfromClass "/Game/BattleBotsContent/Skills/Effects/BP_Link.BP_Link_C" _returnvalue_2))
                (Variables|/Game/BattleBotsContent/Skills/Effects/BP_Link.BP_Link_C|SetSkillUpdater _returnvalue_8 _returnvalue_6)
                (Utilities|Array|Add (Variables|/Game/BattleBotsContent/Skills/BP_Skill.BP_Skill_C|GetOriginalSkillEffectsToApply _returnvalue_2) _returnvalue_8)
                ;;[1 1 1] Initialize the skill properties
                (Default|Initialize _returnvalue_2)
                ;;[1 1 1] Add the skill to the component
                (Utilities|Array|Add (Variables|Default|GetSlottedSkills) _returnvalue_2))
              (:RowNotFound))))))))

(fn HandleSkillModsforEffects
  (params (SkillEffectModClass :type BP%20Skill%20Mod%20Class%20Reference) (Updater :type BP%20Skill%20Updater%20Object%20Reference))
  (bind _asbp_skill_effect_modifier (Utilities|Casting|CastToBP_SkillEffectModifierClass SkillEffectModClass)
    (:then
      (if (>= (Utilities|Array|FindItem (Variables|Default|GetExistingSkillEffectModifierClasses) _asbp_skill_effect_modifier) 0)
        ;[1 1 1] No need to plug in an effect. "Create Effect" will initialize
        (bind _returnvalue (Game|ConstructObjectfromClass _asbp_skill_effect_modifier Updater))
        (Default|CreateEffect _returnvalue (Game|GetGameMode))
        (Utilities|Array|Add (Variables|/Game/BattleBotsContent/Skills/BP_SkillUpdater.BP_SkillUpdater_C|GetSkillMods Updater) _returnvalue)
        (return true)
        (else
          (return false))))
    (:CastFailed
      (return false))))