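; BP_Unit is a grid-battle unit actor that acts as a skill user, with skills and stats held in UnitComponent and team in BPUnitTeamComponent.
; Main and link skills are slots 0 and 1; skill calls only check validity before the skill applies itself to a target or grid cell.
; Game mode interfaces supply grid coordinates and the controlled-unit list it leaves on destruction.
; RespondToSkill and UseSkillInDirection are stubs.
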(event `self.ReceiveBeginPlay`)

(event `self.ReceiveActorBeginOverlap`
  (params (OtherActor :type "Actor Object Reference")))

(event `self.ReceiveTick`
  (params (DeltaSeconds :type "Float (single-precision)")))

(fn `DestroySkillUser`
  (returns (` ` :type Boolean))
  (bind _asbpi_battle_manager (cast `/Game/BattleBotsContent/Global/BPI_BattleManager` (`GameplayStatics.GetGameMode`))
    (:`then`
      (bind _controllableunits (`/Game/BattleBotsContent/Global/BPI_BattleManager.GetControlledUnits` _asbpi_battle_manager))
      (`KismetArrayLibrary.Array_RemoveItem` _controllableunits self)
      (`self.K2_DestroyActor` self)
      (return false))
    (:`CastFailed`
      (`KismetSystemLibrary.PrintString` "BP_Unit::DestroySkillUser: could not cast GameMode to BP_BattleGameMode")
      (return false))))

(fn `GetGridLocation`
  (returns (X :type Integer) (Y :type Integer))
  (bind _asbpi_grid_managing_game_mode (cast `/Game/BattleBotsContent/Grid/BPI_GridManagingGameMode` (`GameplayStatics.GetGameMode`))
    (:`then`
      (bind _gridmanager (`/Game/BattleBotsContent/Grid/BPI_GridManagingGameMode.GetGridManager` _asbpi_grid_managing_game_mode))
      (bind (_gridlocationx _gridlocationy) (`/Game/BattleBotsContent/Grid/BP_GridManager.WorldToGridCoordinates` _gridmanager (`self.K2_GetActorLocation`)))
      (return _gridlocationx _gridlocationy))
    (:`CastFailed`
      (return -1 -1))))

(fn `GetSkills`
  (returns (Skills :type "Array of /Game/BattleBotsContent/Skills/BP_Skill Object Reference"))
  (return (`/Game/BattleBotsContent/Units/BP_UnitComponent.SlottedSkills` (`self.UnitComponent`))))

(fn `GetStats`
  (returns (Stats :type "/Game/BattleBotsContent/Units/BPS_Stats Structure"))
  (return (`/Game/BattleBotsContent/Units/BP_UnitComponent.Stats` (`self.UnitComponent`))))

(fn `GetTeam`
  (returns (Team :type "/Game/BattleBotsContent/Global/ETeamAssociation Enum"))
  (return (`/Game/BattleBotsContent/Units/BP_UnitTeamComponent.Team` (`self.BP_UnitTeamComponent`))))

(fn `GetWorldLocation`
  (returns (WorldLocation :type "Vector Structure"))
  (return (`self.K2_GetActorLocation`)))

(fn `RespondToSkill`
  (params (SkillUsed :type "/Game/BattleBotsContent/Skills/BP_Skill Object Reference"))
  (returns (` ` :type Boolean))
  (return false))

(fn `SetSkills`
  (params (NewSkills :type "Array of /Game/BattleBotsContent/Skills/BP_Skill Object Reference (by ref)"))
  (returns (` ` :type Boolean))
  (set `/Game/BattleBotsContent/Units/BP_UnitComponent.SlottedSkills` NewSkills (`self.UnitComponent`))
  (return false))

(fn `SetStats`
  (params (NewStats :type "/Game/BattleBotsContent/Units/BPS_Stats Structure"))
  (returns (` ` :type Boolean))
  (set `/Game/BattleBotsContent/Units/BP_UnitComponent.Stats` NewStats (`self.UnitComponent`))
  (return false))

(fn `SetWorldLocation`
  (params (NewWorldLocation :type "Vector Structure"))
  (returns (` ` :type Boolean))
  (`self.K2_SetActorLocation` NewWorldLocation false true)
  (return false))

(fn `UseLinkSkillOnTarget`
  (params (TargetedSkillUser :type "/Game/BattleBotsContent/Skills/BPI_SkillUser Interface"))
  (returns (` ` :type Boolean))
  (bind __ (`self.UseSkillOnTarget` (`KismetArrayLibrary.Array_Get` (`/Game/BattleBotsContent/Units/BP_UnitComponent.SlottedSkills` (`self.UnitComponent`)) 1) TargetedSkillUser))
  (return __))

(fn `UseMainSkillOnTarget`
  (params (TargetedSkillUser :type "/Game/BattleBotsContent/Skills/BPI_SkillUser Interface"))
  (returns (` ` :type Boolean))
  (bind __ (`self.UseSkillOnTarget` (`KismetArrayLibrary.Array_Get` (`/Game/BattleBotsContent/Units/BP_UnitComponent.SlottedSkills` (`self.UnitComponent`))) TargetedSkillUser))
  (return __))

(fn `UserConstructionScript`
  (`parent.UserConstructionScript`))

(fn `UseSkillInDirection`
  (params (Skill :type "/Game/BattleBotsContent/Skills/BP_Skill Object Reference") (Direction :type "Rotator Structure"))
  (returns (` ` :type Boolean))
  (return false))

(fn `UseSkillOnGridLocation`
  (params (Skill :type "/Game/BattleBotsContent/Skills/BP_Skill Object Reference") (X :type Integer) (Y :type Integer))
  (returns (` ` :type Boolean))
  (`/Engine/EditorBlueprintResources/StandardMacros.IsValid` Skill
    (:`Is Valid`
      (`/Game/BattleBotsContent/Skills/BP_Skill.ApplySkillToGridLocation` Skill X Y self)
      (return true))
    (:`Is Not Valid`
      (`KismetSystemLibrary.PrintString` "BP_Unit::UseSkillOnGridLocation: Could not locate referenced skill within Slotted Skills")
      (return false))))

(fn `UseSkillOnTarget`
  (params (Skill :type "/Game/BattleBotsContent/Skills/BP_Skill Object Reference") (TargetSkillUser :type "/Game/BattleBotsContent/Skills/BPI_SkillUser Interface"))
  (returns (` ` :type Boolean))
  ;[1 1 1] Determines whether the Skill ref is inside the Unit's skills
  (`/Engine/EditorBlueprintResources/StandardMacros.IsValid` Skill
    (:`Is Valid`
      (`/Game/BattleBotsContent/Skills/BP_Skill.ApplySkillToTarget` Skill self TargetSkillUser)
      (return true))
    (:`Is Not Valid`
      (`KismetSystemLibrary.PrintString` "BP_Unit::UseSkillOnTarget: Could not locate referenced skill within Slotted Skills")
      (return false))))