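; BP_UnitSpawner spawns BattleBots units onto the game's grid.
; SpawnUnit gets the grid manager from the game mode through BPI_GridManagingGameMode and multiplies the grid X and Y by cell size to get a world position at Z zero.
; It spawns the configured UnitClass there, owned by the spawner, then initializes the new actor's UnitComponent with the given unit name.
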(event `self.ReceiveBeginPlay`)

(event `self.ReceiveActorBeginOverlap`
  (params (OtherActor :type "Actor Object Reference")))

(event `self.ReceiveTick`
  (params (DeltaSeconds :type "Float (single-precision)")))

(fn `SpawnUnit`
  (params (UnitName :type Name) (GridLocationX :type Integer) (GridLocationY :type Integer))
  (bind _asbpi_grid_managing_game_mode (cast `/Game/BattleBotsContent/Grid/BPI_GridManagingGameMode` (`GameplayStatics.GetGameMode`)))
  (bind _gridmanager (`/Game/BattleBotsContent/Grid/BPI_GridManagingGameMode.GetGridManager` _asbpi_grid_managing_game_mode))
  (bind _cellsize (`/Game/BattleBotsContent/Grid/BP_Grid.CellSize` (`/Game/BattleBotsContent/Grid/BP_GridManager.Grid` _gridmanager)))
  (bind _returnvalue (`|SpawnActorFromClass` (`self.UnitClass`) (`KismetMathLibrary.Conv_VectorToTransform` (`KismetMathLibrary.MakeVector` (* GridLocationX _cellsize) (* GridLocationY _cellsize))) "Undefined" "OverrideRootScale" self))
  (`/Game/BattleBotsContent/Units/BP_UnitComponent.Initialize` (`/Game/BattleBotsContent/Units/BP_Unit.UnitComponent` _returnvalue) UnitName))

(fn `UserConstructionScript`)