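; BP_Grid is the battle grid, a 2D board of BP_GridCell objects stored in a flat, row-major array.
; Initialize builds the cells from the given dimensions, then copies interactable and terrain names from DT_GridAttributesTable, matching row order to cell index.
; Helper functions convert between cells, indices and X/Y coordinates.
; Units and interactables resolve to their cell through the coordinates on their grid component.
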(event Custom|Initialize
  (params (LengthX :type Integer) (LengthY :type Integer) (CellSize :type Float%20%28single-precision%29))
  ;[1 1 1] Initialize grid properties
  (bind _output_get (Variables|Default|SetLengthX LengthX))
  (bind _output_get_2 (Variables|Default|SetWidthY LengthY))
  (Variables|Default|SetCellSize CellSize)
  (bind _output_get_3 (Variables|Default|SetGridCells (Utilities|Array|MakeArray 0)))
  (Utilities|Array|Clear _output_get_3)
  (for _index (range 0 (- _output_get_2 1))
    (for _index_2 (range 0 (- _output_get 1))
      (bind _returnvalue (Game|ConstructObjectfromClass "/Game/BattleBotsContent/Grid/BP_GridCell.BP_GridCell_C" self))
      (Utilities|Array|Add (Variables|Default|GetGridCells) _returnvalue)))
  (CallFunction|AssignDataTableAttributes))

(fn GetCoordinatesfromGridCell
  (params (Tile :type BP%20Grid%20Cell%20Object%20Reference))
  ;[1 1 1] Given specific tile, return x and y coordinates
  (bind (_xcoordinate _ycoordinate) (CallFunction|GetCoordinatesfromIndex (Utilities|Array|FindItem (Variables|Default|GetGridCells) Tile)))
  (return _xcoordinate _ycoordinate))

(fn GetGridCellfromCoordinates
  (params (X :type Integer) (Y :type Integer))
  ;[1 1 1] Given coordinates for 2D array, calculate where that tile is in 1D array and return it
  (return (Utilities|Array|Get(acopy) (Variables|Default|GetGridCells) (+ (* Y (Variables|Default|GetLengthX)) X))))

(fn GetGridCellfromObject
  (params (Actor :type Actor%20Object%20Reference))
  ;[1 1 1] Cast object to either unit or interactable (only two things that may be on grid) and then calculate which tile they are on according to their coordinates.
  (bind _asbp_unit (Utilities|Casting|CastToBP_Unit Actor)
    (:then
      (bind _tile (CallFunction|GetGridCellfromCoordinates (Variables|/Game/BattleBotsContent/Grid/BP_GridComponent.BP_GridComponent_C|GetXCoordinate (Variables|/Game/BattleBotsContent/Units/BP_Unit.BP_Unit_C|GetBP_GridComponent _asbp_unit)) (Variables|/Game/BattleBotsContent/Grid/BP_GridComponent.BP_GridComponent_C|GetYCoordinate (Variables|/Game/BattleBotsContent/Units/BP_Unit.BP_Unit_C|GetBP_GridComponent _asbp_unit))))
      (LocalVariables|SetTile _tile))
    (:CastFailed
      (bind _asbp_grid_interactable (Utilities|Casting|CastToBP_GridInteractable Actor)
        (:then
          (bind _tile_2 (CallFunction|GetGridCellfromCoordinates (Variables|/Game/BattleBotsContent/Grid/BP_GridComponent.BP_GridComponent_C|GetXCoordinate (Variables|/Game/BattleBotsContent/Grid/BP_GridActor.BP_GridActor_C|GetBP_GridComponent _asbp_grid_interactable)) (Variables|/Game/BattleBotsContent/Grid/BP_GridComponent.BP_GridComponent_C|GetYCoordinate (Variables|/Game/BattleBotsContent/Grid/BP_GridActor.BP_GridActor_C|GetBP_GridComponent _asbp_grid_interactable))))
          (LocalVariables|SetTile _tile_2))
        (:CastFailed
          _))))
  (return (LocalVariables|GetTile)))

(fn GetCoordinatesfromIndex
  (params (Index :type Integer))
  (bind _lengthx (Variables|Default|GetLengthX))
  ;[1 1 1] Given index in 1D array, calculate where x and y coordinates would be in 2D array
  (if (== Index -1)
    (bind _output_get (LocalVariables|SetYCoor -1))
    (LocalVariables|SetXCoor _output_get)
    (else
      (LocalVariables|SetXCoor (Math|Integer|%(Integer) Index _lengthx))
      (LocalVariables|SetYCoor (/ Index _lengthx))))
  (return (LocalVariables|GetXCoor) (LocalVariables|GetYCoor)))

(fn AssignDataTableAttributes
  ;[1 1 1] Assign grid cell's values based on corresponding index in data table
  (bind _outrownames (DataTable|GetDataTableRowNames "/Game/BattleBotsContent/Grid/DT_GridAttributesTable.DT_GridAttributesTable"))
  (for (_array_element _array_index) _outrownames
    (bind _returnvalue (Utilities|GetDataTableRow "/Game/BattleBotsContent/Grid/DT_GridAttributesTable.DT_GridAttributesTable" _array_element)
      (:then
        (Variables|/Game/BattleBotsContent/Grid/BP_GridCell.BP_GridCell_C|SetInteractableName (Utilities|Array|Get(acopy) (Variables|Default|GetGridCells) _array_index) (Utilities|Struct|BreakBPS_InteractableAttributes (.Interactable (Utilities|Struct|BreakBPS_GridCellAttributes _returnvalue))))
        (Variables|/Game/BattleBotsContent/Grid/BP_GridCell.BP_GridCell_C|SetTerrainName (Utilities|Array|Get(acopy) (Variables|Default|GetGridCells) _array_index) (Utilities|Struct|BreakBPS_TerrainAttributes (.Terrain (Utilities|Struct|BreakBPS_GridCellAttributes _returnvalue)))))))
  (return))